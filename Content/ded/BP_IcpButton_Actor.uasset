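; Actor hosting an ICP button widget that links its Enter press to a target T-ILS DED display, apparently for cockpit code entry.
; On BeginPlay it casts its widget to BP_IcpButton, clears its WidgetInteraction reference and binds the Enter event.
; Enter only casts the display's widget to BP_DED_T-ILS.
; The check comparing entered text with GoalText and printing the result is disconnected.
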(event `self.ReceiveBeginPlay`
  (bind _asbp_icp_button (cast `/Game/ded/BP_IcpButton` (`WidgetComponent.GetUserWidgetObject` (`self.Widget`))))
  (set `self.WidgetInteraction` null)
  (add `/Game/ded/BP_IcpButton.enter pressed` _asbp_icp_button (delegate `enter pressed_Event_0`)))

(event `enter pressed_Event_0`
  (bind _asbp_ded_t_ils (cast `/Game/ded/dedpage/BP_DED_T-ILS` (`WidgetComponent.GetUserWidgetObject` (`/Game/ded/dedpage/BP_DED_T-ILS_Actor.Widget` (`self.TargetDisplay`))))))

(fn `UserConstructionScript`)