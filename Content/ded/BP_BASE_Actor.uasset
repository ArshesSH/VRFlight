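; Actor that manages the pages of a DED display (main page, list, DEST 1–5, OA1, T-ILS), each a widget on a child actor.
; BeginPlay caches each page's widget from its WidgetComponent and hides all but the main page.
; Per-page functions show or hide widgets using boolean flags and nested checks, with most DEST pages gated on the list flag.
; Several DEST3–5 functions set another page's flag, so tracked state can drift from actual visibility.
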(event `self.ReceiveBeginPlay`
  (`self.On Initialize dest UI`)
  (`self.On List Initialize UI`)
  (`self.On Mainpage Initialize UI`)
  (`self.On oa1 Initialize UI`)
  (`self.On T-ILS Initialize UI`)
  (`self.On Initialize dest2 UI`)
  (`self.On Initialize dest4 UI`)
  (`self.On Initialize dest5 UI`)
  (`self.On Initialize dest3 UI`))

(fn `On DEST UI`
  (bind _bp_destwidget_ref (`self.BP DESTWidget Ref`))
  (if (`self.is listshow`)
    (if (`self.is destshow`)
      (`Widget.SetVisibility` _bp_destwidget_ref "Hidden")
      (set `self.is destshow` false)
      (else
        (`Widget.SetVisibility` _bp_destwidget_ref "Visible")
        (set `self.is destshow` true)
        (if (`self.is mainpageshow`)
          (`Widget.SetVisibility` (`self.BP DESTWidget Ref`) "Hidden")
          (set `self.is mainpageshow` false)
          (if (`self.is listshow`)
            _
            (else
              _))
          (`Widget.SetVisibility` (`self.BP listWidget Ref`) "Hidden")
          (set `self.is listshow` false)
          (if (`self.is DEST2Show`)
            (`Widget.SetVisibility` (`self.BP DEST2Widget Ref`) "Hidden")
            (set `self.is DEST2Show` false)))))))

(fn `On DEST2down UI`
  (if (`self.is listshow`)
    (if (`self.is DEST2Show`)
      (`Widget.SetVisibility` (`self.BP DEST2Widget Ref`) "Hidden")
      (set `self.is DEST2Show` false)
      (else
        (`Widget.SetVisibility` (`self.BP DEST2Widget Ref`) "Hidden")
        (set `self.is DEST2Show` false)))
    (if (`self.is mainpageshow`)
      (`Widget.SetVisibility` (`self.BP MainpageWidget Ref`) "Hidden")
      (set `self.is mainpageshow` false)
      (if (`self.is listshow`)
        _
        (else
          _))
      (`Widget.SetVisibility` (`self.BP listWidget Ref`) "Hidden")
      (set `self.is listshow` false)
      (if (`self.is destshow`)
        (`Widget.SetVisibility` (`self.BP DESTWidget Ref`) "Hidden")
        (set `self.is destshow` false)))))

(fn `On DEST2up UI`
  (bind _bp_dest2widget_ref (`self.BP DEST2Widget Ref`))
  (if (`self.is listshow`)
    (if (`self.is DEST2Show`)
      (`Widget.SetVisibility` _bp_dest2widget_ref "Hidden")
      (set `self.is DEST2Show` false)
      (else
        (`Widget.SetVisibility` _bp_dest2widget_ref "Visible")
        (set `self.is DEST2Show` true)
        (if (`self.is mainpageshow`)
          (`Widget.SetVisibility` (`self.BP MainpageWidget Ref`) "Hidden")
          (set `self.is mainpageshow` false)
          (if (`self.is listshow`)
            _
            (else
              _))
          (`Widget.SetVisibility` (`self.BP listWidget Ref`) "Hidden")
          (set `self.is listshow` false)
          (if (`self.is destshow`)
            (`Widget.SetVisibility` (`self.BP DESTWidget Ref`) "Hidden")
            (set `self.is destshow` false)))))))

(fn `On DEST3downUI`
  (if (`self.is listshow`)
    (if (`self.is DEST3Show`)
      (`Widget.SetVisibility` (`self.BP DEST3Widget Ref`) "Hidden")
      (set `self.is DEST2Show` false)
      (if (`self.is mainpageshow`)
        (`Widget.SetVisibility` (`self.BP MainpageWidget Ref`) "Hidden")
        (set `self.is mainpageshow` false)
        (if (`self.is listshow`)
          _
          (else
            _))
        (`Widget.SetVisibility` (`self.BP listWidget Ref`) "Hidden")
        (set `self.is listshow` false)
        (if (`self.is destshow`)
          (`Widget.SetVisibility` (`self.BP DESTWidget Ref`) "Hidden")
          (set `self.is destshow` false)
          (if (`self.is DEST2Show`)
            (`Widget.SetVisibility` (`self.BP DEST2Widget Ref`) "Hidden")
            (set `self.is DEST2Show` false))))
      (else
        (`KismetSystemLibrary.PrintString` "Hello")))))

(fn `On DEST3up UI`
  (if (`self.is listshow`)
    (if (not (`self.is DEST3Show`))
      (`KismetSystemLibrary.PrintString` "Hello"))
    (`Widget.SetVisibility` (`self.BP DEST3Widget Ref`) "Visible")
    (set `self.is DEST3Show` true)
    (if (`self.is mainpageshow`)
      (`Widget.SetVisibility` (`self.BP MainpageWidget Ref`) "Hidden")
      (set `self.is mainpageshow` false)
      (if (`self.is listshow`)
        _
        (else
          _))
      (`Widget.SetVisibility` (`self.BP listWidget Ref`) "Hidden")
      (set `self.is listshow` false)
      (if (`self.is destshow`)
        _
        (else
          _))
      (`Widget.SetVisibility` (`self.BP DESTWidget Ref`) "Hidden")
      (set `self.is destshow` false)
      (if (`self.is DEST2Show`)
        (`Widget.SetVisibility` (`self.BP DEST2Widget Ref`) "Hidden")
        (set `self.is DEST2Show` false)))))

(fn `On DEST4downUI`
  (if (`self.is listshow`)
    (if (`self.is DEST4Show`)
      _
      (else
        _))
    (`Widget.SetVisibility` (`self.BP DEST4Widget Ref`) "Hidden")
    (set `self.is DEST2Show` false)
    (if (`self.is mainpageshow`)
      (`Widget.SetVisibility` (`self.BP MainpageWidget Ref`) "Hidden")
      (set `self.is mainpageshow` false)
      (if (`self.is listshow`)
        _
        (else
          _))
      (`Widget.SetVisibility` (`self.BP listWidget Ref`) "Hidden")
      (set `self.is listshow` false)
      (if (`self.is destshow`)
        (`Widget.SetVisibility` (`self.BP DESTWidget Ref`) "Hidden")
        (set `self.is destshow` false)
        (if (`self.is DEST2Show`)
          (`Widget.SetVisibility` (`self.BP DEST2Widget Ref`) "Hidden")
          (set `self.is DEST2Show` false)
          (if (`self.is DEST3Show`)
            (`Widget.SetVisibility` (`self.BP DEST3Widget Ref`) "Hidden")
            (set `self.is DEST3Show` false)))))))

(fn `On DEST4up UI`
  (if (`self.is listshow`)
    (if (not (`self.is DEST4Show`))
      (`KismetSystemLibrary.PrintString` "Hello"))
    (`Widget.SetVisibility` (`self.BP DEST4Widget Ref`) "Visible")
    (set `self.is DEST4Show` true)
    (if (`self.is mainpageshow`)
      (`Widget.SetVisibility` (`self.BP MainpageWidget Ref`) "Hidden")
      (set `self.is mainpageshow` false)
      (if (`self.is listshow`)
        _
        (else
          _))
      (`Widget.SetVisibility` (`self.BP listWidget Ref`) "Hidden")
      (set `self.is listshow` false)
      (if (`self.is destshow`)
        _
        (else
          _))
      (`Widget.SetVisibility` (`self.BP DESTWidget Ref`) "Hidden")
      (set `self.is destshow` false)
      (if (`self.is DEST2Show`)
        (`Widget.SetVisibility` (`self.BP DEST2Widget Ref`) "Hidden")
        (set `self.is DEST2Show` false)
        (if (`self.is DEST3Show`)
          (`Widget.SetVisibility` (`self.BP DEST3Widget Ref`) "Hidden")
          (set `self.is DEST3Show` false))))))

(fn `On DEST5downUI`
  (if (`self.is listshow`)
    (if (`self.is DEST5Show`)
      _
      (else
        _))
    (`Widget.SetVisibility` (`self.BP DEST5Widget Ref`) "Hidden")
    (set `self.is DEST2Show` false)
    (if (`self.is mainpageshow`)
      (`Widget.SetVisibility` (`self.BP MainpageWidget Ref`) "Hidden")
      (set `self.is mainpageshow` false)
      (if (`self.is listshow`)
        _
        (else
          _))
      (`Widget.SetVisibility` (`self.BP listWidget Ref`) "Hidden")
      (set `self.is listshow` false)
      (if (`self.is destshow`)
        (`Widget.SetVisibility` (`self.BP DESTWidget Ref`) "Hidden")
        (set `self.is destshow` false)
        (if (`self.is DEST2Show`)
          (`Widget.SetVisibility` (`self.BP DEST2Widget Ref`) "Hidden")
          (set `self.is DEST2Show` false)
          (if (`self.is DEST3Show`)
            (`Widget.SetVisibility` (`self.BP DEST3Widget Ref`) "Hidden")
            (set `self.is DEST3Show` false)
            (if (`self.is DEST4Show`)
              (`Widget.SetVisibility` (`self.BP DEST4Widget Ref`) "Hidden")
              (set `self.is DEST4Show` false))))))))

(fn `On DEST5up UI`
  (if (`self.is listshow`)
    (if (not (`self.is DEST5Show`))
      (`KismetSystemLibrary.PrintString` "Hello"))
    (`Widget.SetVisibility` (`self.BP DEST5Widget Ref`) "Visible")
    (set `self.is DEST4Show` true)
    (if (`self.is mainpageshow`)
      (`Widget.SetVisibility` (`self.BP MainpageWidget Ref`) "Hidden")
      (set `self.is mainpageshow` false)
      (if (`self.is listshow`)
        _
        (else
          _))
      (`Widget.SetVisibility` (`self.BP listWidget Ref`) "Hidden")
      (set `self.is listshow` false)
      (if (`self.is destshow`)
        _
        (else
          _))
      (`Widget.SetVisibility` (`self.BP DESTWidget Ref`) "Hidden")
      (set `self.is destshow` false)
      (if (`self.is DEST2Show`)
        (`Widget.SetVisibility` (`self.BP DEST2Widget Ref`) "Hidden")
        (set `self.is DEST2Show` false)
        (if (`self.is DEST3Show`)
          (`Widget.SetVisibility` (`self.BP DEST3Widget Ref`) "Hidden")
          (set `self.is DEST3Show` false)
          (if (`self.is DEST4Show`)
            (`Widget.SetVisibility` (`self.BP DEST4Widget Ref`) "Hidden")
            (set `self.is DEST4Show` false)))))))

(fn `On Initialize dest UI`
  (bind _asbp_ded_dest (cast `/Game/ded/dedpage/DESTWAYPOINT/BP_DED_DEST` (`WidgetComponent.GetUserWidgetObject` (`self.GetComponentByClass` (`ChildActorComponent.ChildActor` (`self.bp_ded_dest_actor`)) "/Script/UMG.WidgetComponent"))))
  (bind _output_get (set `self.BP DESTWidget Ref` _asbp_ded_dest))
  (`/Engine/EditorBlueprintResources/StandardMacros.IsValid` _output_get
    (:`Is Valid`
      (set `self.is destshow` false)
      (`Widget.SetVisibility` (`self.BP DESTWidget Ref`) "Hidden"))
    (:`Is Not Valid`
      (`KismetSystemLibrary.PrintString` "initialize err"))))

(fn `On Initialize dest2 UI`
  (bind _asbp_ded_dest2 (cast `/Game/ded/dedpage/DESTWAYPOINT/BP_DED_DEST2` (`WidgetComponent.GetUserWidgetObject` (`self.GetComponentByClass` (`ChildActorComponent.ChildActor` (`self.bp_ded_dest2_actor`)) "/Script/UMG.WidgetComponent"))))
  (bind _output_get (set `self.BP DEST2Widget Ref` _asbp_ded_dest2))
  (`/Engine/EditorBlueprintResources/StandardMacros.IsValid` _output_get
    (:`Is Valid`
      (set `self.is DEST2Show` false)
      (`Widget.SetVisibility` (`self.BP DEST2Widget Ref`) "Hidden"))
    (:`Is Not Valid`
      (`KismetSystemLibrary.PrintString` "initialize err"))))

(fn `On Initialize dest3 UI`
  (bind _asbp_ded_dest3 (cast `/Game/ded/dedpage/DESTWAYPOINT/BP_DED_DEST3` (`WidgetComponent.GetUserWidgetObject` (`self.GetComponentByClass` (`ChildActorComponent.ChildActor` (`self.bp_ded_dest3_actor`)) "/Script/UMG.WidgetComponent"))))
  (bind _output_get (set `self.BP DEST3Widget Ref` _asbp_ded_dest3))
  (`/Engine/EditorBlueprintResources/StandardMacros.IsValid` _output_get
    (:`Is Valid`
      (set `self.is DEST3Show` false)
      (`Widget.SetVisibility` (`self.BP DEST3Widget Ref`) "Hidden"))
    (:`Is Not Valid`
      (`KismetSystemLibrary.PrintString` "initialize err"))))

(fn `On Initialize dest4 UI`
  (bind _asbp_ded_dest4 (cast `/Game/ded/dedpage/DESTWAYPOINT/BP_DED_DEST4` (`WidgetComponent.GetUserWidgetObject` (`self.GetComponentByClass` (`ChildActorComponent.ChildActor` (`self.bp_ded_dest4_actor`)) "/Script/UMG.WidgetComponent"))))
  (bind _output_get (set `self.BP DEST4Widget Ref` _asbp_ded_dest4))
  (`/Engine/EditorBlueprintResources/StandardMacros.IsValid` _output_get
    (:`Is Valid`
      (set `self.is DEST4Show` false)
      (`Widget.SetVisibility` (`self.BP DEST4Widget Ref`) "Hidden"))
    (:`Is Not Valid`
      (`KismetSystemLibrary.PrintString` "initialize err"))))

(fn `On Initialize dest5 UI`
  (bind _asbp_ded_dest5 (cast `/Game/ded/dedpage/DESTWAYPOINT/BP_DED_DEST5` (`WidgetComponent.GetUserWidgetObject` (`self.GetComponentByClass` (`ChildActorComponent.ChildActor` (`self.bp_ded_dest5_actor`)) "/Script/UMG.WidgetComponent"))))
  (bind _output_get (set `self.BP DEST5Widget Ref` _asbp_ded_dest5))
  (`/Engine/EditorBlueprintResources/StandardMacros.IsValid` _output_get
    (:`Is Valid`
      (set `self.is DEST5Show` false)
      (`Widget.SetVisibility` (`self.BP DEST5Widget Ref`) "Hidden"))
    (:`Is Not Valid`
      (`KismetSystemLibrary.PrintString` "initialize err"))))

(fn `On List Initialize UI`
  (locals (NewLocalVar_0 :type "Object Object Reference") (NewLocalVar_1 :type "/Game/ded/dedpage/BP_DED_LIST Object Reference"))
  (bind _asbp_ded_list (cast `/Game/ded/dedpage/BP_DED_LIST` (`WidgetComponent.GetUserWidgetObject` (`self.GetComponentByClass` (`ChildActorComponent.ChildActor` (`self.bp_ded_list_actor1`)) "/Script/UMG.WidgetComponent"))))
  (bind _output_get (set `self.BP listWidget Ref` _asbp_ded_list))
  (`/Engine/EditorBlueprintResources/StandardMacros.IsValid` _output_get
    (:`Is Valid`
      (set `self.is listshow` false)
      (`Widget.SetVisibility` (`self.BP listWidget Ref`) "Hidden"))
    (:`Is Not Valid`
      (`KismetSystemLibrary.PrintString` "initialize err"))))

(fn `On list UI`
  (bind _bp_listwidget_ref (`self.BP listWidget Ref`))
  (if (`self.is listshow`)
    (`Widget.SetVisibility` _bp_listwidget_ref "Hidden")
    (set `self.is listshow` false)
    (if (not (`self.is listshow`))
      (`Widget.SetVisibility` (`self.BP MainpageWidget Ref`) "Visible")
      (set `self.is mainpageshow` false))
    (else
      (`Widget.SetVisibility` _bp_listwidget_ref "Visible")
      (set `self.is listshow` true)
      (if (`self.is listshow`)
        (`Widget.SetVisibility` (`self.BP MainpageWidget Ref`) "Hidden")
        (set `self.is mainpageshow` false)))))

(fn `On Mainpage Initialize UI`
  (locals (NewLocalVar_0 :type "Object Object Reference") (NewLocalVar_1 :type "/Game/ded/dedpage/BP_DED_LIST Object Reference"))
  (bind _asbp_ded_mainpage (cast `/Game/ded/dedpage/BP_DED_Mainpage` (`WidgetComponent.GetUserWidgetObject` (`self.GetComponentByClass` (`ChildActorComponent.ChildActor` (`self.bp_ded_mainpage_actor`)) "/Script/UMG.WidgetComponent"))))
  (bind _output_get (set `self.BP MainpageWidget Ref` _asbp_ded_mainpage))
  (`/Engine/EditorBlueprintResources/StandardMacros.IsValid` _output_get
    (:`Is Valid`
      (set `self.is mainpageshow` true))
    (:`Is Not Valid`
      (`KismetSystemLibrary.PrintString` "initialize err"))))

(fn `On Mainpage UI`
  (if (`self.is mainpageshow`)
    (`KismetSystemLibrary.PrintString` "err")
    (if (`self.is DEST2Show`)
      (`Widget.SetVisibility` (`self.BP DEST2Widget Ref`) "Hidden")
      (set `self.is DEST2Show` false)
      (if (`self.is destshow`)
        (`Widget.SetVisibility` (`self.BP DESTWidget Ref`) "Hidden")
        (set `self.is destshow` false)))
    (else
      (`Widget.SetVisibility` (`self.BP MainpageWidget Ref`) "Visible")
      (set `self.is mainpageshow` true)
      (if (`self.is mainpageshow`)
        (`Widget.SetVisibility` (`self.BP oa1Widget Ref`) "Hidden")
        (set `self.is oa1show` false)
        (if (`self.is listshow`)
          (`Widget.SetVisibility` (`self.BP listWidget Ref`) "Hidden")
          (set `self.is listshow` false)
          (if (`self.is destshow`)
            (`Widget.SetVisibility` (`self.BP DESTWidget Ref`) "Hidden")
            (set `self.is destshow` false)
            (if (`self.is T-ILSshow`)
              (`Widget.SetVisibility` (`self.BP T-ILSWidget Ref`) "Hidden")
              (set `self.is T-ILSshow` false)
              (if (`self.is DEST2Show`)
                (`Widget.SetVisibility` (`self.BP DEST2Widget Ref`) "Hidden")
                (set `self.is DEST2Show` false)))))))))

(fn `On oa1 Initialize UI`
  (locals (NewLocalVar_0 :type "Object Object Reference") (NewLocalVar_1 :type "/Game/ded/dedpage/BP_DED_LIST Object Reference"))
  (bind _asbp_ded_oa1 (cast `/Game/ded/dedpage/BP_DED_OA1` (`WidgetComponent.GetUserWidgetObject` (`self.GetComponentByClass` (`ChildActorComponent.ChildActor` (`self.bp_ded_oa1_actor`)) "/Script/UMG.WidgetComponent"))))
  (bind _output_get (set `self.BP oa1Widget Ref` _asbp_ded_oa1))
  (`/Engine/EditorBlueprintResources/StandardMacros.IsValid` _output_get
    (:`Is Valid`
      (set `self.is oa1show` false)
      (`Widget.SetVisibility` (`self.BP oa1Widget Ref`) "Hidden"))
    (:`Is Not Valid`
      (`KismetSystemLibrary.PrintString` "initialize err"))))

(fn `On OA1 UI`
  (bind _bp_oa1widget_ref (`self.BP oa1Widget Ref`))
  (if (`self.is destshow`)
    (if (`self.is oa1show`)
      (`Widget.SetVisibility` _bp_oa1widget_ref "Hidden")
      (set `self.is oa1show` false)
      (else
        (`Widget.SetVisibility` _bp_oa1widget_ref "Visible")
        (set `self.is oa1show` true)
        (if (`self.is destshow`)
          (`Widget.SetVisibility` (`self.BP DESTWidget Ref`) "Hidden")
          (set `self.is destshow` false))))
    (else
      (`KismetSystemLibrary.PrintString` "ON OA1 ERR"))))

(fn `On T-ILS Initialize UI`
  (locals (NewLocalVar_0 :type "Object Object Reference") (NewLocalVar_1 :type "/Game/ded/dedpage/BP_DED_LIST Object Reference"))
  (bind _asbp_ded_t_ils (cast `/Game/ded/dedpage/BP_DED_T-ILS` (`WidgetComponent.GetUserWidgetObject` (`self.GetComponentByClass` (`ChildActorComponent.ChildActor` (`self.bp_ded_T-ILS_actor`)) "/Script/UMG.WidgetComponent"))))
  (bind _output_get (set `self.BP T-ILSWidget Ref` _asbp_ded_t_ils))
  (`/Engine/EditorBlueprintResources/StandardMacros.IsValid` _output_get
    (:`Is Valid`
      (set `self.is T-ILSshow` false)
      (`Widget.SetVisibility` (`self.BP T-ILSWidget Ref`) "Hidden"))
    (:`Is Not Valid`
      (`KismetSystemLibrary.PrintString` "initialize err"))))

(fn `On T-ILS UI`
  (bind _bp_t_ilswidget_ref (`self.BP T-ILSWidget Ref`))
  (if (`self.is T-ILSshow`)
    (`Widget.SetVisibility` _bp_t_ilswidget_ref "Hidden")
    (set `self.is T-ILSshow` false)
    (else
      (`Widget.SetVisibility` _bp_t_ilswidget_ref "Visible")
      (set `self.is T-ILSshow` true)
      (if (`self.is mainpageshow`)
        _
        (else
          _))
      (`Widget.SetVisibility` (`self.BP MainpageWidget Ref`) "Hidden")
      (set `self.is mainpageshow` false))))

(fn `UserConstructionScript`)