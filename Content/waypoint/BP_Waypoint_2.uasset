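; Second-numbered waypoint actor that hands off to BP_Waypoint_3 when the F-16C reaches it.
; On BeginPlay it finds and stores the BP_Waypoint_3 instance in the level.
; When BP_F-16C overlaps its Box, it hides its Widget and Sphere, disables itself, then enables the next waypoint and shows that Sphere.
; The overlap does not check IsWaypointEnabled, and the next waypoint's Widget is left untouched.
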(event `self.ReceiveBeginPlay`
  (bind _outactors (`GameplayStatics.GetAllActorsOfClass` "/Game/waypoint/BP_Waypoint_3.BP_Waypoint_3_C"))
  (for _array_element _outactors
    (set `self.Waypoint3` _array_element)))

(event `self.Box.OnComponentBeginOverlap`
  (params (OverlappedComponent :type "PrimitiveComponent Object Reference") (OtherActor :type "Actor Object Reference") (OtherComp :type "PrimitiveComponent Object Reference") (OtherBodyIndex :type Integer) (bFromSweep :type Boolean) (SweepResult :type "HitResult Structure (by ref)"))
  (bind _waypoint3 (`self.Waypoint3`))
  (cast `/Game/Asset/F-16C/BP_F-16C` OtherActor)
  (`SceneComponent.SetVisibility` (`self.Widget`) false false)
  (`SceneComponent.SetVisibility` (`self.Sphere`) false false)
  (set `self.bIsWaypointEnabled` false)
  (set `/Game/waypoint/BP_Waypoint_3.bIsWaypointEnabled` true _waypoint3)
  (`SceneComponent.SetVisibility` (`/Game/waypoint/BP_Waypoint_3.Sphere` _waypoint3) true false))

(fn `UserConstructionScript`)