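; Cockpit waypoint indicator for the F-16C that shows a widget pointing toward the active waypoint or the airport ILS.
; BeginPlay caches the five waypoint actors, the ILS actor and the player's F-16C.
; While main power is on, Tick picks the first enabled waypoint and swaps its widget in; ILS mode also shows the airport widget.
; SetWidgetLocation turns yaw and pitch differences to the target into clamped offsets of one shared moving point.
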(event `self.ReceiveBeginPlay`
  (`|ExecutionSequence`
    (:`then_0`
      (bind _outactors (`GameplayStatics.GetAllActorsOfClass` "/Game/waypoint/BP_Waypoint.BP_Waypoint_C"))
      (for _array_element _outactors
        (set `self.Waypoint1` _array_element)))
    (:`then_1`
      (bind _outactors_2 (`GameplayStatics.GetAllActorsOfClass` "/Game/waypoint/BP_Waypoint_2.BP_Waypoint_2_C"))
      (for _array_element_2 _outactors_2
        (set `self.Waypoint2` _array_element_2)))
    (:`then_2`
      (bind _outactors_3 (`GameplayStatics.GetAllActorsOfClass` "/Game/waypoint/BP_Waypoint_3.BP_Waypoint_3_C"))
      (for _array_element_3 _outactors_3
        (set `self.Waypoint3` _array_element_3)))
    (:`then_3`
      (bind _outactors_4 (`GameplayStatics.GetAllActorsOfClass` "/Game/waypoint/BP_Waypoint_4.BP_Waypoint_4_C"))
      (for _array_element_4 _outactors_4
        (set `self.Waypoint4` _array_element_4)))
    (:`then_4`
      (bind _outactors_5 (`GameplayStatics.GetAllActorsOfClass` "/Game/waypoint/BP_Waypoint_5.BP_Waypoint_5_C"))
      (for _array_element_5 _outactors_5
        (set `self.Waypoint5` _array_element_5)))
    (:`then_5`
      (bind _outactors_6 (`GameplayStatics.GetAllActorsOfClass` "/Game/Flight_Instrument_Pack/Widgets/InstrumentWidgets/HSI_Widget/BP_ILS.BP_ILS_C"))
      (for _array_element_6 _outactors_6
        (set `self.ILSInstrument` _array_element_6)))
    (:`then_6`
      (bind _asbp_f_16c (cast `/Game/Asset/F-16C/BP_F-16C` (`GameplayStatics.GetPlayerPawn` 0)))
      (set `self.F-16` _asbp_f_16c))))

(event `self.ReceiveTick`
  (params (DeltaSeconds :type "Float (single-precision)"))
  (if (`/Game/Asset/F-16C/BP_F-16C.bMainPowerOn` (`self.F-16`))
    (`|ExecutionSequence`
      (:`then_0`
        (if (`/Game/waypoint/BP_Waypoint.bIsWaypointEnabled` (`self.Waypoint1`))
          (`self.SetWidgetLocation` (`/Game/waypoint/BP_Waypoint.Scene` (`self.Waypoint1`)))
          (`/Engine/EditorBlueprintResources/StandardMacros.DoOnce` false
            (:`Completed`
              (`SceneComponent.SetVisibility` (`self.WaypointWidget_1`) true false)))
          (elif (`/Game/waypoint/BP_Waypoint_2.bIsWaypointEnabled` (`self.Waypoint2`))
            (`self.SetWidgetLocation` (`/Game/waypoint/BP_Waypoint_2.Scene` (`self.Waypoint2`)))
            (`/Engine/EditorBlueprintResources/StandardMacros.DoOnce` false
              (:`Completed`
                (`SceneComponent.SetVisibility` (`self.WaypointWidget_1`) false false)
                (`SceneComponent.SetVisibility` (`self.WaypointWidget_2`) true false)))
            (elif (`/Game/waypoint/BP_Waypoint_3.bIsWaypointEnabled` (`self.Waypoint3`))
              (`self.SetWidgetLocation` (`/Game/waypoint/BP_Waypoint_3.Scene` (`self.Waypoint3`)))
              (`/Engine/EditorBlueprintResources/StandardMacros.DoOnce` false
                (:`Completed`
                  (`SceneComponent.SetVisibility` (`self.WaypointWidget_2`) false false)
                  (`SceneComponent.SetVisibility` (`self.WaypointWidget_3`) true false)))
              (elif (`/Game/waypoint/BP_Waypoint_4.bIsWaypointEnabled` (`self.Waypoint4`))
                (`self.SetWidgetLocation` (`/Game/waypoint/BP_Waypoint_4.Scene` (`self.Waypoint4`)))
                (`/Engine/EditorBlueprintResources/StandardMacros.DoOnce` false
                  (:`Completed`
                    (`SceneComponent.SetVisibility` (`self.WaypointWidget_3`) false false)
                    (`SceneComponent.SetVisibility` (`self.WaypointWidget_4`) true false)))
                (elif (`/Game/waypoint/BP_Waypoint_5.bIsWaypointEnabled` (`self.Waypoint5`))
                  (`self.SetWidgetLocation` (`/Game/waypoint/BP_Waypoint_5.Scene` (`self.Waypoint5`)))
                  (`/Engine/EditorBlueprintResources/StandardMacros.DoOnce` false
                    (:`Completed`
                      (`SceneComponent.SetVisibility` (`self.WaypointWidget_4`) false false)
                      (`SceneComponent.SetVisibility` (`self.WaypointWidget_5`) true false)))
                  (else
                    (`SceneComponent.SetVisibility` (`self.WaypointWidget_1`) false false)
                    (`SceneComponent.SetVisibility` (`self.WaypointWidget_2`) false false)
                    (`SceneComponent.SetVisibility` (`self.WaypointWidget_3`) false false)
                    (`SceneComponent.SetVisibility` (`self.WaypointWidget_4`) false false)
                    (`SceneComponent.SetVisibility` (`self.WaypointWidget_5`) false false))))))))
      (:`then_1`
        (if (`/Game/Asset/F-16C/BP_F-16C.bILSOn` (`self.F-16`))
          (`self.SetWidgetLocation` (`/Game/Flight_Instrument_Pack/Widgets/InstrumentWidgets/HSI_Widget/BP_ILS.Position` (`self.ILSInstrument`)))
          (`SceneComponent.SetVisibility` (`self.WaypointWidget_Airport`) true false)
          (else
            (`SceneComponent.SetVisibility` (`self.WaypointWidget_Airport`) false false)))))))

(fn `SetWidgetLocation`
  (params (TargetWaypointScene :type "SceneComponent Object Reference"))
  (bind (_returnvalue_roll _returnvalue_pitch _returnvalue_yaw) (`KismetMathLibrary.BreakRotator` (`SceneComponent.K2_GetComponentRotation` (`local.TargetWaypointScene`))))
  (bind (_returnvalue_roll_2 _returnvalue_pitch_2 _returnvalue_yaw_2) (`KismetMathLibrary.BreakRotator` (`SceneComponent.K2_GetComponentRotation` (`Actor.RootComponent` (`GameplayStatics.GetPlayerPawn` 0)))))
  (`SceneComponent.K2_SetRelativeRotation` (`local.TargetWaypointScene`) (`KismetMathLibrary.FindLookAtRotation` (`SceneComponent.K2_GetComponentLocation` (`Actor.RootComponent` (`GameplayStatics.GetPlayerPawn` 0))) (`SceneComponent.K2_GetComponentLocation` (`local.TargetWaypointScene`))) false false)
  (`SceneComponent.K2_SetRelativeLocation` (`self.WidgetMovingPoint`) (`KismetMathLibrary.MakeVector` 0.0 (`KismetMathLibrary.FClamp` (- _returnvalue_yaw_2 _returnvalue_yaw) -45.0 45.0) (`KismetMathLibrary.FClamp` (- _returnvalue_pitch _returnvalue_pitch_2) -45.0 45.0)) false false))

(fn `UserConstructionScript`)