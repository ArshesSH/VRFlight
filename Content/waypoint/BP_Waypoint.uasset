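; BP_Waypoint is a waypoint that hands off to a BP_Waypoint_2 when the player-type jet BP_F-16C flies into it.
; On BeginPlay it finds all BP_Waypoint_2 actors and keeps the last one as the next waypoint.
; A Box overlap by the F-16C disables this waypoint and hides its Sphere, then enables and shows the next one.
; The overlap does not check whether this waypoint is currently enabled.
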(event `self.ReceiveBeginPlay`
  (bind _outactors (`GameplayStatics.GetAllActorsOfClass` "/Game/waypoint/BP_Waypoint_2.BP_Waypoint_2_C"))
  (for _array_element _outactors
    (set `self.Waypoint2` _array_element)))

(event `self.Box.OnComponentBeginOverlap`
  (params (OverlappedComponent :type "PrimitiveComponent Object Reference") (OtherActor :type "Actor Object Reference") (OtherComp :type "PrimitiveComponent Object Reference") (OtherBodyIndex :type Integer) (bFromSweep :type Boolean) (SweepResult :type "HitResult Structure (by ref)"))
  (bind _waypoint2 (`self.Waypoint2`))
  (cast `/Game/Asset/F-16C/BP_F-16C` OtherActor)
  (set `self.bIsWaypointEnabled` false)
  (`SceneComponent.SetVisibility` (`self.Sphere`) false false)
  (set `/Game/waypoint/BP_Waypoint_2.bIsWaypointEnabled` true _waypoint2)
  (`SceneComponent.SetVisibility` (`/Game/waypoint/BP_Waypoint_2.Sphere` _waypoint2) true false))

(fn `UserConstructionScript`)