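; Flyable Ju87 showcase pawn that registers with a nearby first-person character, shows a HUD while possessed, and spawns a new character on exit.
; AeroComp drag, thrust, lift and weathervane components act on the airframe, with throttle also driving propeller spin and audio.
; Temporary flight controls apply torque scaled by speed and mass, damping pitch input by angle of attack.
; Non-authority input is forwarded through events; the camera toggles between first and third person.
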(event `self.ReceiveTick`
  (params (DeltaSeconds :type "Float (single-precision)"))
  (bind _propeller (`self.propeller`))
  (bind _propeller_2 (`self.propeller`))
  (bind _ju87 (`self.Ju87`))
  (bind _throttle (`/Game/AeroComp/AeroComps/AeroComp_THRUSTER.throttle` (`self.AeroComp_THRUSTER`)))
  (bind _relativerotation (`SceneComponent.RelativeRotation` (`self.jujuProp`)))
  (`|ExecutionSequence`
    (:`then_0`
      ;[0.505 1 0.6082] Various cosmetic stuff
      (`|ExecutionSequence`
        (:`then_0`
          (if (`self.isPlayerNear`)
            (`SceneComponent.K2_SetWorldRotation` (`self.Info`) (`KismetMathLibrary.FindLookAtRotation` (`SceneComponent.K2_GetComponentLocation` (`self.Info`)) (`self.K2_GetActorLocation` (`self.player`))) false false)))
        (:`then_1`
          (`SceneComponent.K2_SetRelativeRotation` (`self.jujuProp`) (`KismetMathLibrary.RInterpTo` _relativerotation (`KismetMathLibrary.MakeRotator` (+ (.roll _relativerotation) 17.0) (.pitch _relativerotation) (.yaw _relativerotation)) (`GameplayStatics.GetWorldDeltaSeconds`) (* (`KismetMathLibrary.FClamp` (`/Game/AeroComp/AeroComps/AeroComp_THRUSTER.throttle` (`self.AeroComp_THRUSTER`)) 0.0001) 150.0)) false false))
        (:`then_2`
          (if (> (`/Game/AeroComp/AeroComps/AeroComp_THRUSTER.throttle` (`self.AeroComp_THRUSTER`)) 0.0)
            (if (not (`AudioComponent.IsPlaying` (`self.propeller`)))
              (`AudioComponent.Play` _propeller 0.0))
            (`AudioComponent.SetPitchMultiplier` _propeller_2 (`KismetMathLibrary.FInterpTo` (`AudioComponent.PitchMultiplier` _propeller_2) (`KismetMathLibrary.Lerp` 0.3 1.2 _throttle) (`GameplayStatics.GetWorldDeltaSeconds`) 1.0))
            (`AudioComponent.SetVolumeMultiplier` _propeller (`KismetMathLibrary.FClamp` _throttle 0.0 0.7))
            (else
              (`AudioComponent.Stop`))))))
    (:`then_1`
      ;[1 1 1] Actor Logging (temp)
      (bind `_α` (`/Game/AeroComp/UtilsAndLibs/AeroUtilityFunctionLibrary.getComponentAOA` _ju87)))
    (:`then_2`
      (bind _velocity (`/Game/AeroComp/UtilsAndLibs/AeroUtilityFunctionLibrary.getComponentVelocity` _ju87)))
    (:`then_3`
      (bind _returnvalue (`PrimitiveComponent.GetPhysicsLinearVelocity` "None"))
      (`SceneComponent.K2_SetWorldRotation` (`self.Arrow`) (`KismetMathLibrary.MakeRotFromX` _returnvalue) false false))))

(event `self.Sphere.OnComponentBeginOverlap`
  (params (OverlappedComponent :type "PrimitiveComponent Object Reference") (OtherActor :type "Actor Object Reference") (OtherComp :type "PrimitiveComponent Object Reference") (OtherBodyIndex :type Integer) (bFromSweep :type Boolean) (SweepResult :type "HitResult Structure (by ref)"))
  ;[1 1 1] Show/Hide info and enable/disable input on player begin/end overlap
  (bind _asfirst_person_character (cast `/Game/AeroComp/FirstPerson/Blueprints/FirstPersonCharacter` OtherActor))
  (set `self.player` _asfirst_person_character)
  (set `self.isPlayerNear` true)
  (`SceneComponent.SetVisibility` (`self.Info`) true false)
  (`/Game/AeroComp/FirstPerson/Blueprints/FirstPersonCharacter.registerPawn` (`self.player`) self))

(event `self.Sphere.OnComponentEndOverlap`
  (params (OverlappedComponent :type "PrimitiveComponent Object Reference") (OtherActor :type "Actor Object Reference") (OtherComp :type "PrimitiveComponent Object Reference") (OtherBodyIndex :type Integer))
  ;[1 1 1] Show/Hide info and enable/disable input on player begin/end overlap
  (cast `/Game/AeroComp/FirstPerson/Blueprints/FirstPersonCharacter` OtherActor)
  (set `self.isPlayerNear` false)
  (`SceneComponent.SetVisibility` (`self.Info`) false false)
  (`/Game/AeroComp/FirstPerson/Blueprints/FirstPersonCharacter.registerPawn` (`self.player`) null))

(event `InputAction|ControlPawn`
  (params (Key :type "Key Structure"))
  ;[1 1 1] Unpossess this actor and spawn back the player
  (:`Pressed`
    (`/Engine/EditorBlueprintResources/ActorMacros.Switch Has Authority`
      (:`Authority`
        (bind _returnvalue (`|SpawnActorFromClass` "/Game/AeroComp/FirstPerson/Blueprints/FirstPersonCharacter.FirstPersonCharacter_C" (`SceneComponent.K2_GetComponentToWorld` (`self.spawnLoc`)) "AdjustIfPossibleButAlwaysSpawn" "OverrideRootScale" null null :!label _label))
        (`Controller.Possess` (`self.GetController`) _returnvalue))
      (:`Remote`
        (`self.unposessJu87`)))))

(event `unposessJu87`
  ;[1 1 1] Unpossess this actor and spawn back the player
  (goto _label))

(event `InputAxis|LookUp`
  (params (AxisValue :type "Float (single-precision)"))
  (bind _returnvalue (* AxisValue -2.0))
  (bind (_relativerotation_roll _relativerotation_pitch _relativerotation_yaw) (`KismetMathLibrary.BreakRotator` (`SceneComponent.RelativeRotation` (`self.Camera`))))
  (bind (_relativerotation_roll_2 _relativerotation_pitch_2 _relativerotation_yaw_2) (`KismetMathLibrary.BreakRotator` (`SceneComponent.RelativeRotation` (`self.SpringArm`))))
  ;[1 1 1] Camera controls
  (if (`self.isFPV`)
    (bind _returnvalue_2 (* (stale `InputAxis|Turn` AxisValue) 2.0))
    (`SceneComponent.K2_SetRelativeRotation` (`KismetMathLibrary.MakeRotator` _relativerotation_roll (`KismetMathLibrary.FClamp` (+ _relativerotation_pitch _returnvalue) -80.0 80.0) (`KismetMathLibrary.FClamp` (+ _relativerotation_yaw _returnvalue_2) -120.0 120.0)))
    (else
      (`SceneComponent.K2_SetRelativeRotation` (`KismetMathLibrary.MakeRotator` _relativerotation_roll_2 (`KismetMathLibrary.FClamp` (+ _relativerotation_pitch_2 _returnvalue) -80.0 80.0) (`KismetMathLibrary.FClamp` (+ _returnvalue_2 _relativerotation_yaw_2) -120.0 120.0))))))

(event `InputAction|Camera toggle`
  (params (Key :type "Key Structure"))
  ;[1 1 1] First/Third person toggle
  (:`Pressed`
    (`/Engine/EditorBlueprintResources/StandardMacros.FlipFlop`
      (:`A`
        (set `self.isFPV` true)
        (`SceneComponent.K2_AttachTo` (`self.Camera`) (`self.FPV`) "None" "SnapToTarget" true))
      (:`B`
        (set `self.isFPV` false)
        (`SceneComponent.K2_AttachTo` (`self.Camera`) (`self.SpringArm`) "SpringEndpoint" "SnapToTarget" true)))))

(event `InputAxis|Turn`
  (params (AxisValue :type "Float (single-precision)"))
  ;[1 1 1] Camera controls
)

(event `self.ReceivePossessed`
  (params (NewController :type "Controller Object Reference"))
  (bind _returnvalue (`|CreateWidget` "/Game/AeroComp/Showcase/Materials/AircraftHUD.AircraftHUD_C"))
  (`UserWidget.AddToViewport` _returnvalue 0))

(event `self.ReceiveUnpossessed`
  (params (OldController :type "Controller Object Reference"))
  (`Widget.RemoveFromParent` (stale `self.ReceivePossessed` _returnvalue)))

(event `InputAxis|Throttle`
  (params (AxisValue :type "Float (single-precision)"))
  ;[1 1 1] Throttle
  (`/Engine/EditorBlueprintResources/ActorMacros.Switch Has Authority`
    (:`Authority`
      (`self.adjustThrottle` AxisValue))
    (:`Remote`
      (`self.adjustThrottleEvent` AxisValue))))

(event `adjustThrottleEvent`
  (params (delta :type "Float (double-precision)"))
  ;[1 1 1] Throttle
  (`self.adjustThrottle` delta))

(event `InputAxis|MoveForward`
  (params (AxisValue :type "Float (single-precision)"))
  (bind _returnvalue (`KismetMathLibrary.Abs` AxisValue))
  ;[1 0.385 0.385] Flight controls (temp)
  (bind `_α` (`/Game/AeroComp/UtilsAndLibs/AeroUtilityFunctionLibrary.getComponentAOA` (`self.Ju87`)))
  (`/Engine/EditorBlueprintResources/ActorMacros.Switch Has Authority`
    (:`Authority`
      (bind _returnvalue_2 (`KismetMathLibrary.FClamp` (* (- _returnvalue (/ (`KismetMathLibrary.Abs` `_α`) 40.0)) (`KismetMathLibrary.SignOfFloat` AxisValue)) -1.0))
      (bind _returnvalue_3 (`KismetMathLibrary.SelectFloat` 0.1 _returnvalue_2 (and (< (`KismetMathLibrary.Abs` _returnvalue_2) 0.1) (> _returnvalue 0.0))))
      (set `self.pitchInput` _returnvalue_3)
      (bind _velocity (`/Game/AeroComp/UtilsAndLibs/AeroUtilityFunctionLibrary.getComponentVelocity` (`self.Ju87`) :!label _label_2))
      (`PrimitiveComponent.AddTorque` (`KismetMathLibrary.GreaterGreater_VectorRotator` (`KismetMathLibrary.MakeVector` 0.0 (* _velocity (`self.pitchSens`) (`self.pitchInput`) (`PrimitiveComponent.GetMass`))) (`self.K2_GetActorRotation`))))
    (:`Remote`
      (`self.inputMoveFwdEvent` _returnvalue_3))))

(event `inputMoveFwdEvent`
  (params (axisValue :type "Float (double-precision)"))
  ;[1 0.385 0.385] Flight controls (temp)
  (set `self.pitchInput` axisValue)
  (goto _label_2))

(event `InputAxis|MoveRight`
  (params (AxisValue :type "Float (single-precision)"))
  ;[1 0.385 0.385] Flight controls (temp)
  (`/Engine/EditorBlueprintResources/ActorMacros.Switch Has Authority`
    (:`Authority`
      (set `self.rollInput` AxisValue)
      (bind _velocity (`/Game/AeroComp/UtilsAndLibs/AeroUtilityFunctionLibrary.getComponentVelocity` (`self.Ju87`) :!label _label_3))
      (`PrimitiveComponent.AddTorque` (`KismetMathLibrary.GreaterGreater_VectorRotator` (`KismetMathLibrary.MakeVector` (* _velocity -30.0 (`self.rollInput`) (`PrimitiveComponent.GetMass`))) (`self.K2_GetActorRotation`))))
    (:`Remote`
      (`self.inputMoveRightEvent` AxisValue))))

(event `inputMoveRightEvent`
  (params (axisValue :type "Float (double-precision)"))
  ;[1 0.385 0.385] Flight controls (temp)
  (set `self.rollInput` axisValue)
  (goto _label_3))

(event `InputAxis|YawRight`
  (params (AxisValue :type "Float (single-precision)"))
  ;[1 0.385 0.385] Flight controls (temp)
  (`/Engine/EditorBlueprintResources/ActorMacros.Switch Has Authority`
    (:`Authority`
      (set `self.yawInput` AxisValue)
      (bind _velocity (`/Game/AeroComp/UtilsAndLibs/AeroUtilityFunctionLibrary.getComponentVelocity` (`self.Ju87`) :!label _label_4))
      (`PrimitiveComponent.AddTorque` (`KismetMathLibrary.GreaterGreater_VectorRotator` (`KismetMathLibrary.MakeVector` 0.0 0.0 (* _velocity 20.0 (`self.yawInput`) (`PrimitiveComponent.GetMass`))) (`self.K2_GetActorRotation`))))
    (:`Remote`
      (`self.inputYawRightEvent` AxisValue))))

(event `inputYawRightEvent`
  (params (axisValue :type "Float (double-precision)"))
  ;[1 0.385 0.385] Flight controls (temp)
  (set `self.yawInput` axisValue)
  (goto _label_4))

(event `self.Ju87.OnComponentHit`
  (params (HitComponent :type "PrimitiveComponent Object Reference") (OtherActor :type "Actor Object Reference") (OtherComp :type "PrimitiveComponent Object Reference") (NormalImpulse :type "Vector Structure") (Hit :type "HitResult Structure (by ref)")))

(fn `adjustThrottle`
  (params (delta :type "Float (double-precision)"))
  (bind _throttle (`/Game/AeroComp/AeroComps/AeroComp_THRUSTER.throttle` (`self.AeroComp_THRUSTER`)))
  (set `/Game/AeroComp/AeroComps/AeroComp_THRUSTER.throttle` (`KismetMathLibrary.FClamp` (`KismetMathLibrary.FInterpTo` _throttle (+ delta _throttle) (`GameplayStatics.GetWorldDeltaSeconds`) 0.15)) (`self.AeroComp_THRUSTER`)))

(fn `getAOA`
  (returns (aoa :type "Float (double-precision)") (sideSlip :type "Float (double-precision)"))
  (bind (`_α` `_β`) (`/Game/AeroComp/UtilsAndLibs/AeroUtilityFunctionLibrary.getComponentAOA` (`self.Ju87`)))
  (return `_α` `_β`))

(fn `getThrottle`
  (returns (throttle :type "Float (double-precision)"))
  (return (`/Game/AeroComp/AeroComps/AeroComp_THRUSTER.throttle` (`self.AeroComp_THRUSTER`))))

(fn `UserConstructionScript`
  (bind _ju87 (`self.Ju87`))
  (`|ExecutionSequence`
    (:`then_0`
      (set `/Game/AeroComp/AeroComps/AeroComp_DRAG.dragComponent` _ju87 (`self.AeroComp_DRAG`)))
    (:`then_1`
      (set `/Game/AeroComp/AeroComps/AeroComp_THRUSTER.thrustComponent` _ju87 (`self.AeroComp_THRUSTER`)))
    (:`then_2`
      (set `/Game/AeroComp/AeroComps/AeroComp_LIFT.liftComponent` _ju87 (`self.AeroComp_LIFT`)))
    (:`then_3`
      (set `/Game/AeroComp/AeroComps/AeroComp_WEATHERVANE.targetComponent` _ju87 (`self.AeroComp_WEATHERVANE`)))))