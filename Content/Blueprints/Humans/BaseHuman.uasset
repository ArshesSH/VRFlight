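; Base human character that serves as either a VR-capable player pawn or a pedestrian with a randomized look.
; Construction picks a random mesh and material, and possession sets controller-driven rotation for PC_HumanController or movement-oriented rotation for other controllers.
; With an HMD enabled, player possession spawns motion controllers, sets up trace and world interactors, switches cameras and hides the body from its owner.
; Fast-moving vehicle overlaps trigger a timed-lifespan ragdoll.
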(event `self.ReceivePossessed`
  (params (NewController :type "Controller Object Reference"))
  (bind _charactermovement (`self.CharacterMovement`))
  (bind _charactermovement_2 (`self.CharacterMovement`))
  (cast `/Game/Blueprints/Controllers/PC_HumanController` NewController
    (:`then`
      (set `self.bUseControllerRotationYaw` true)
      (set `CharacterMovementComponent.bUseControllerDesiredRotation` true _charactermovement_2)
      (set `CharacterMovementComponent.bOrientRotationToMovement` false _charactermovement_2)
      (if (`HeadMountedDisplayFunctionLibrary.IsHeadMountedDisplayEnabled`)
        (`self.SetUpVRPawn`)))
    (:`CastFailed`
      (set `self.bUseControllerRotationYaw` false)
      (set `CharacterMovementComponent.bUseControllerDesiredRotation` false _charactermovement)
      (set `CharacterMovementComponent.bOrientRotationToMovement` true _charactermovement))))

(event `self.CapsuleComponent.OnComponentBeginOverlap`
  (params (OverlappedComponent :type "PrimitiveComponent Object Reference") (OtherActor :type "Actor Object Reference") (OtherComp :type "PrimitiveComponent Object Reference") (OtherBodyIndex :type Integer) (bFromSweep :type Boolean) (SweepResult :type "HitResult Structure (by ref)"))
  (bind _asbase_vehicle (cast `/Game/Blueprints/Vehicles/BaseVehicle` OtherActor))
  (if (> (`KismetMathLibrary.VSize` (`self.GetVelocity` _asbase_vehicle)) 250.0)
    (`self.Ragdoll`)))

(event `Ragdoll`
  (bind _mesh (`self.Mesh`))
  (`PrimitiveComponent.SetCollisionEnabled` _mesh "QueryAndPhysics")
  (`PrimitiveComponent.SetSimulatePhysics` _mesh true)
  (`SceneComponent.K2_DetachFromComponent` _mesh "KeepWorld" "KeepWorld" "KeepWorld" true)
  (`PrimitiveComponent.SetCollisionEnabled` (`self.CapsuleComponent`) "NoCollision")
  (`self.SetLifeSpan` 15.0))

(fn `SetRandomMaterial`
  (bind _materialtouse (`self.MaterialToUse`))
  (`PrimitiveComponent.SetMaterial` (`self.Mesh`) 0 (`|GetArrayItem` _materialtouse (`KismetMathLibrary.RandomIntegerInRange` 0 (`KismetArrayLibrary.Array_LastIndex` _materialtouse)))))

(fn `SetRandomMesh`
  (bind _meshtouse (`self.MeshToUse`))
  (`SkinnedMeshComponent.SetSkinnedAssetAndUpdate` (`self.Mesh`) (`|GetArrayItem` _meshtouse (`KismetMathLibrary.RandomIntegerInRange` 0 (`KismetArrayLibrary.Array_LastIndex` _meshtouse))) true))

(fn `SetUpVRPawn`
  (bind _returnvalue (`KismetMathLibrary.MakeTransform` (0.0 0.0 0.0)))
  (bind _returnvalue_2 (`self.GetController`))
  (`|ExecutionSequence`
    (:`then_0`
      (bind _returnvalue_3 (`|SpawnActorFromClass` "/Game/ExampleContent/VR_Trace_Interaction/Blueprints/BP_TraceVisualiser.BP_TraceVisualiser_C" _returnvalue "Undefined" "OverrideRootScale" null 1.0 (1.0 1.0 1.0) null))
      (`/Game/ExampleContent/VR_Trace_Interaction/Blueprints/Components/BP_TraceInteractor.Setup` (`self.BP_TraceInteractor_L`) _returnvalue_3 self "NewEnumerator2" true (`self.WidgetInteraction`))
      (bind _returnvalue_4 (`|SpawnActorFromClass` "/Game/ExampleContent/VR_Trace_Interaction/Blueprints/BP_TraceVisualiser.BP_TraceVisualiser_C" (`KismetMathLibrary.MakeTransform` (0.0 0.0 0.0)) "Undefined" "OverrideRootScale" null 1.0 (1.0 1.0 1.0) null))
      (`/Game/ExampleContent/VR_Trace_Interaction/Blueprints/Components/BP_TraceInteractor.Setup` (`self.BP_TraceInteractor_R`) _returnvalue_4 self "NewEnumerator2" true (`self.WidgetInteraction`))
      (`/Game/ExampleContent/VR_World_Interaction/Blueprints/Components/BPC_WorldInteractor.Setup` (`self.BPC_WorldInteractor_L`) (`self.L_Hand_Sphere`))
      (`/Game/ExampleContent/VR_World_Interaction/Blueprints/Components/BPC_WorldInteractor.Setup` (`self.BPC_WorldInteractor_R`) (`self.R_Hand_Sphere`)))
    (:`then_1`
      (bind _returnvalue_5 (`|SpawnActorFromClass` "/Game/VirtualRealityBP/Blueprints/BP_MotionController.BP_MotionController_C" _returnvalue "Undefined" "OverrideRootScale" _returnvalue_2 "Left" null))
      (`self.K2_AttachToComponent` _returnvalue_5 (`self.Scene`) "None" "SnapToTarget" "SnapToTarget" "SnapToTarget" false)
      (bind _aspc_human_controller (cast `/Game/Blueprints/Controllers/PC_HumanController` (`self.GetController`)))
      (set `/Game/Blueprints/Controllers/PC_HumanController.LeftHand` _returnvalue_5 _aspc_human_controller))
    (:`then_2`
      (bind _returnvalue_6 (`|SpawnActorFromClass` "/Game/VirtualRealityBP/Blueprints/BP_MotionController.BP_MotionController_C" _returnvalue "Undefined" "OverrideRootScale" _returnvalue_2 "Right" null))
      (`self.K2_AttachToComponent` _returnvalue_6 (`self.Scene`) "None" "SnapToTarget" "SnapToTarget" "SnapToTarget" false)
      (bind _aspc_human_controller_2 (cast `/Game/Blueprints/Controllers/PC_HumanController` (`self.GetController`)))
      (set `/Game/Blueprints/Controllers/PC_HumanController.RightHand` _returnvalue_6 _aspc_human_controller_2))
    (:`then_3`
      (`ActorComponent.Deactivate` (`self.Camera`))
      (`ActorComponent.Activate` (`self.Camera1`) false)
      (`PrimitiveComponent.SetOwnerNoSee` (`self.Mesh`) true))))

(fn `UserConstructionScript`
  (`self.SetRandomMesh`)
  (`self.SetRandomMaterial`))