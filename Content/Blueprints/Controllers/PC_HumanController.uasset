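; Player controller that switches the player between human, vehicle and aircraft pawns, routing movement, zoom and VR interaction input to whichever is controlled.
; ControlPawn enters a camera-traced vehicle or possesses the human's PawnToPossess, destroying the human; exiting spawns a new one.
; Aircraft swaps branch on authority, with remote calling separate possess/unpossess events.
; While the right hand grips the steering wheel, Tick maps its lateral offset to steering.
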(event `InputAxis|Turn`
  (params (AxisValue :type "Float (single-precision)"))
  ;[1 1 1] Mouse Look
  (`self.AddYawInput` AxisValue))

(event `InputAxis|LookUp`
  (params (AxisValue :type "Float (single-precision)"))
  ;[1 1 1] Mouse Look
  (`self.AddPitchInput` AxisValue))

(event `Key|R`
  (params (Key :type "Key Structure"))
  (:`Pressed`
    (`HeadMountedDisplayFunctionLibrary.ResetOrientationAndPosition` 0.0)))

(event `Key|MouseScrollUp`
  (params (Key :type "Key Structure"))
  ;[1 1 1] Toggle View
  (:`Pressed`
    (if (`self.ControllingVehicle`)
      (`/Game/Blueprints/Vehicles/BaseVehicle.ZoomIn` (`self.ControlledVehicle`))
      (elif (`self.ControllingAircraft`)
        (`/Game/Blueprints/Vehicles/BP_BaseAirplane.ZoomIn` (`self.ControlledAircraft`))))))

(event `Key|MouseScrollDown`
  (params (Key :type "Key Structure"))
  ;[1 1 1] Toggle View
  (:`Pressed`
    (if (`self.ControllingVehicle`)
      (`/Game/Blueprints/Vehicles/BaseVehicle.ZoomOut` (`self.ControlledVehicle`))
      (elif (`self.ControllingAircraft`)
        (`/Game/Blueprints/Vehicles/BP_BaseAirplane.ZoomOut` (`self.ControlledAircraft`))))))

(event `self.ReceiveBeginPlay`
  (bind _returnvalue (`self.K2_GetPawn`))
  (bind _asbase_vehicle (cast `/Game/Blueprints/Vehicles/BaseVehicle` _returnvalue)
    (:`then`
      (set `self.ControlledVehicle` _asbase_vehicle)
      (set `self.ControllingVehicle` true)
      (set `self.ControllingHuman` false)
      (set `self.ControllingHuman` false))
    (:`CastFailed`
      (bind _asbp_base_airplane (cast `/Game/Blueprints/Vehicles/BP_BaseAirplane` _returnvalue)
        (:`then`
          (set `self.ControlledAircraft` _asbp_base_airplane)
          (set `self.ControllingVehicle` false)
          (set `self.ControllingHuman` false)
          (set `self.ControllingAircraft` true))
        (:`CastFailed`
          (bind _asbase_human (cast `/Game/Blueprints/Humans/BaseHuman` _returnvalue))
          (set `self.ControlledHuman` _asbase_human)
          (set `self.ControllingVehicle` false)
          (set `self.ControllingHuman` true)
          (set `self.ControllingAircraft` false)))))
  (`KismetSystemLibrary.Delay` 0.2)
  (if (`HeadMountedDisplayFunctionLibrary.IsHeadMountedDisplayEnabled`)
    (`self.SetUpVR`)))

(event `posesspawn`
  (if (`KismetSystemLibrary.IsValid` (`/Game/Blueprints/Humans/BaseHuman.pawnToPossess` (`self.ControlledHuman`))) :!label _label
    (`self.Possess` (`/Game/Blueprints/Humans/BaseHuman.pawnToPossess` (`self.ControlledHuman`)))
    (`self.K2_DestroyActor` (`self.ControlledHuman`))
    (set `self.ControllingAircraft` true)
    (set `self.ControllingHuman` false)
    (bind _asbp_base_airplane (cast `/Game/Blueprints/Vehicles/BP_BaseAirplane` (`self.K2_GetPawn`)))
    (set `self.ControlledAircraft` _asbp_base_airplane)))

(event `InputAxis|MoveForward`
  (params (AxisValue :type "Float (single-precision)"))
  (bind _controlledhuman (`self.ControlledHuman`))
  ;[1 1 1] Movement
  (if (`self.ControllingVehicle`)
    (`WheeledVehicleMovementComponent.SetThrottleInput` (`WheeledVehicle.VehicleMovement` (`self.ControlledVehicle`)) AxisValue)
    (elif (`self.ControllingHuman`)
      (`Pawn.AddMovementInput` _controlledhuman (`self.GetActorForwardVector` _controlledhuman) AxisValue false)
      (elif (`self.ControllingAircraft`)
        (`/Game/Blueprints/Vehicles/BP_BaseAirplane.Throttle` (`self.ControlledAircraft`) AxisValue)))))

(event `InputAction|ControlPawn`
  (params (Key :type "Key Structure"))
  (bind _returnvalue_location (`KismetMathLibrary.BreakTransform` (`SceneComponent.K2_GetComponentToWorld` (`/Game/Blueprints/Vehicles/BP_BaseAirplane.spawnLoc` (`self.ControlledAircraft`)))))
  (:`Pressed`
    (if (`self.ControllingHuman`)
      (bind (_hit_actor _isvehiclenear) (`self.CheckVehicleToDrive`))
      (if _isvehiclenear
        (`self.EnterVehicle` _hit_actor)
        (else
          (`/Engine/EditorBlueprintResources/ActorMacros.Switch Has Authority` ; Has Authority to Aircraft?
            (:`Authority`
              (goto _label))
            (:`Remote`
              (`self.posesspawn`)))))
      (elif (`self.ControllingVehicle`)
        (`self.LeaveVehicle`)
        (elif (`self.ControllingAircraft`)
          (`/Engine/EditorBlueprintResources/ActorMacros.Switch Has Authority`
            (:`Authority`
              (bind _returnvalue (`|SpawnActorFromClass` "/Game/Blueprints/Humans/Human_PlayerPawn.Human_PlayerPawn_C" (`KismetMathLibrary.MakeTransform` _returnvalue_location) "AdjustIfPossibleButAlwaysSpawn" "OverrideRootScale" null null :!label _label_2))
              (`self.Possess` _returnvalue)
              (set `self.ControlledHuman` _returnvalue)
              (set `self.ControllingAircraft` false)
              (set `self.ControllingHuman` true))
            (:`Remote`
              (`self.unposess`))))))))

(event `InputAction|Jump`
  (params (Key :type "Key Structure"))
  (bind _controlledhuman (`self.ControlledHuman`))
  ;[1 1 1] Movement
  (:`Pressed`
    (if (`self.ControllingHuman`)
      (`Character.Jump` _controlledhuman)))
  (:`Released`
    (if (`self.ControllingHuman`)
      (`Character.StopJumping` _controlledhuman))))

(event `InputAxis|MoveRight`
  (params (AxisValue :type "Float (single-precision)"))
  (bind _controlledhuman (`self.ControlledHuman`))
  (bind _controlledvehicle (`self.ControlledVehicle`))
  ;[1 1 1] Movement
  (if (`self.ControllingVehicle`)
    (if (not (`/Game/Blueprints/Vehicles/BaseVehicle.IsGrippingWheel` _controlledvehicle))
      (`WheeledVehicleMovementComponent.SetSteeringInput` (`WheeledVehicle.VehicleMovement` _controlledvehicle) AxisValue)
      (set `/Game/Blueprints/Vehicles/BaseVehicle.Steering` AxisValue _controlledvehicle))
    (elif (`self.ControllingHuman`)
      (`/Engine/EditorBlueprintResources/StandardMacros.IsValid` _controlledhuman
        (:`Is Valid`
          (`Pawn.AddMovementInput` _controlledhuman (`self.GetActorRightVector` _controlledhuman) AxisValue false)))
      (elif (`self.ControllingAircraft`)
        (`/Game/Blueprints/Vehicles/BP_BaseAirplane.RudderInput` (`self.ControlledAircraft`) AxisValue)))))

(event `unposess`
  (goto _label_2))

(event `InputAction|GrabRight`
  (params (Key :type "Key Structure"))
  (bind _righthand (`self.RightHand`))
  (bind _righthand_2 (`self.RightHand`))
  (bind _controllingvehicle (`self.ControllingVehicle`))
  (bind _controlledvehicle (`self.ControlledVehicle`))
  (bind _returnvalue (`SceneComponent.K2_GetComponentLocation` (`/Game/VirtualRealityBP/Blueprints/BP_MotionController.HandMesh` (`self.RightHand`))))
  ;[1 1 1] Grip Wheel
  (:`Pressed`
    (if _controllingvehicle
      (if (< (`KismetMathLibrary.VSize` (- (`SceneComponent.GetSocketLocation` (`WheeledVehicle.Mesh` _controlledvehicle) "SteeringW") _returnvalue)) 35.0)
        (set `/Game/Blueprints/Vehicles/BaseVehicle.IsGrippingWheel` true _controlledvehicle)
        (set `self.HandLocationOnGrab` _returnvalue)
        (set `/Game/VirtualRealityBP/Blueprints/BP_MotionController.bWantsToGrip` true _righthand_2)
        (else
          (set `/Game/Blueprints/Vehicles/BaseVehicle.IsGrippingWheel` false _controlledvehicle)
          (set `/Game/VirtualRealityBP/Blueprints/BP_MotionController.bWantsToGrip` true _righthand_2)))
      (else
        (set `/Game/VirtualRealityBP/Blueprints/BP_MotionController.bWantsToGrip` true _righthand))))
  (:`Released`
    (if _controllingvehicle
      (set `/Game/Blueprints/Vehicles/BaseVehicle.IsGrippingWheel` false _controlledvehicle)
      (set `/Game/VirtualRealityBP/Blueprints/BP_MotionController.bWantsToGrip` false (`self.RightHand`))
      (else
        (`/Game/VirtualRealityBP/Blueprints/BP_MotionController.ReleaseActor` _righthand)))))

(event `self.ReceiveTick`
  (params (DeltaSeconds :type "Float (single-precision)"))
  (bind _controlledvehicle (`self.ControlledVehicle`))
  (bind _controlledvehicle_2 (`self.ControlledVehicle`))
  (bind _returnvalue (`self.GetTransform` _controlledvehicle_2))
  (bind (_returnvalue_x _returnvalue_y) (`KismetMathLibrary.BreakVector` (- (`KismetMathLibrary.InverseTransformLocation` _returnvalue (`SceneComponent.K2_GetComponentLocation` (`/Game/VirtualRealityBP/Blueprints/BP_MotionController.HandMesh` (`self.RightHand`)))) (`KismetMathLibrary.InverseTransformLocation` _returnvalue (`SceneComponent.GetSocketLocation` (`WheeledVehicle.Mesh` _controlledvehicle_2) "SteeringW")))))
  (bind _returnvalue_2 (`KismetMathLibrary.MapRangeClamped` _returnvalue_y -25.0 25.0 -1.0 1.0))
  (if (`self.ControllingVehicle`)
    (if (`/Game/Blueprints/Vehicles/BaseVehicle.IsGrippingWheel` (`self.ControlledVehicle`))
      (`WheeledVehicleMovementComponent.SetSteeringInput` (`WheeledVehicle.VehicleMovement` _controlledvehicle) _returnvalue_2)
      (set `/Game/Blueprints/Vehicles/BaseVehicle.Steering` _returnvalue_2 _controlledvehicle))))

(event `InputAction|Motioncontroller_Left_Thumbstick`
  (params (Key :type "Key Structure"))
  (bind _bp_traceinteractor_l (`/Game/Blueprints/Humans/BaseHuman.BP_TraceInteractor_L` (`self.ControlledHuman`)))
  (:`Pressed`
    (if (not (`self.ControllingVehicle`))
      (`/Engine/EditorBlueprintResources/StandardMacros.IsValid` (`self.ControlledHuman`)
        (:`Is Valid`
          (`/Game/ExampleContent/VR_Trace_Interaction/Blueprints/Components/BP_TraceInteractor.ActivateEventDown` _bp_traceinteractor_l)))))
  (:`Released`
    (if (not (`self.ControllingVehicle`))
      (`/Engine/EditorBlueprintResources/StandardMacros.IsValid` (`self.ControlledHuman`)
        (:`Is Valid`
          (`/Game/ExampleContent/VR_Trace_Interaction/Blueprints/Components/BP_TraceInteractor.ActivateEventUp` _bp_traceinteractor_l))))))

(event `InputAction|Motioncontroller_Right_Thumbstick`
  (params (Key :type "Key Structure"))
  (bind _bp_traceinteractor_r (`/Game/Blueprints/Humans/BaseHuman.BP_TraceInteractor_R` (`self.ControlledHuman`)))
  (:`Pressed`
    (if (not (`self.ControllingVehicle`))
      (`/Engine/EditorBlueprintResources/StandardMacros.IsValid` (`self.ControlledHuman`)
        (:`Is Valid`
          (`/Game/ExampleContent/VR_Trace_Interaction/Blueprints/Components/BP_TraceInteractor.ActivateEventDown` _bp_traceinteractor_r)))))
  (:`Released`
    (if (not (`self.ControllingVehicle`))
      (`/Engine/EditorBlueprintResources/StandardMacros.IsValid` (`self.ControlledHuman`)
        (:`Is Valid`
          (`/Game/ExampleContent/VR_Trace_Interaction/Blueprints/Components/BP_TraceInteractor.ActivateEventUp` _bp_traceinteractor_r))))))

(event `InputAction|Motioncontroller_Left_Trigger`
  (params (Key :type "Key Structure"))
  (bind _bpc_worldinteractor_l (`/Game/Blueprints/Humans/BaseHuman.BPC_WorldInteractor_L` (`self.ControlledHuman`)))
  (:`Pressed`
    (if (not (`self.ControllingVehicle`))
      (`/Engine/EditorBlueprintResources/StandardMacros.IsValid` (`self.ControlledHuman`)
        (:`Is Valid`
          (`/Game/ExampleContent/VR_World_Interaction/Blueprints/Components/BPC_WorldInteractor.UsePressed` _bpc_worldinteractor_l)))))
  (:`Released`
    (if (not (`self.ControllingVehicle`))
      (`/Engine/EditorBlueprintResources/StandardMacros.IsValid` (`self.ControlledHuman`)
        (:`Is Valid`
          (`/Game/ExampleContent/VR_World_Interaction/Blueprints/Components/BPC_WorldInteractor.UseReleased` _bpc_worldinteractor_l))))))

(event `InputAction|MotionController_Right_Trigger`
  (params (Key :type "Key Structure"))
  (bind _bpc_worldinteractor_r (`/Game/Blueprints/Humans/BaseHuman.BPC_WorldInteractor_R` (`self.ControlledHuman`)))
  (:`Pressed`
    (if (not (`self.ControllingVehicle`))
      (`/Engine/EditorBlueprintResources/StandardMacros.IsValid` (`self.ControlledHuman`)
        (:`Is Valid`
          (`/Game/ExampleContent/VR_World_Interaction/Blueprints/Components/BPC_WorldInteractor.UsePressed` _bpc_worldinteractor_r)))))
  (:`Released`
    (if (not (`self.ControllingVehicle`))
      (`/Engine/EditorBlueprintResources/StandardMacros.IsValid` (`self.ControlledHuman`)
        (:`Is Valid`
          (`/Game/ExampleContent/VR_World_Interaction/Blueprints/Components/BPC_WorldInteractor.UseReleased` _bpc_worldinteractor_r))))))

(event `InputAction|GrabLeft`
  (params (Key :type "Key Structure"))
  (bind _lefthand (`self.LeftHand`))
  (bind _bpc_worldinteractor_l (`/Game/Blueprints/Humans/BaseHuman.BPC_WorldInteractor_L` (`self.ControlledHuman`)))
  (:`Pressed`
    (`/Engine/EditorBlueprintResources/StandardMacros.IsValid` (`self.ControlledHuman`)
      (:`Is Valid`
        (`/Game/ExampleContent/VR_World_Interaction/Blueprints/Components/BPC_WorldInteractor.PickupPressed` _bpc_worldinteractor_l)
        (`/Game/ExampleContent/VR_World_Interaction/Blueprints/Components/BPC_WorldInteractor.DragStart` _bpc_worldinteractor_l))
      (:`Is Not Valid`
        _))
    (`/Game/VirtualRealityBP/Blueprints/BP_MotionController.GrabActor` _lefthand))
  (:`Released`
    (`/Engine/EditorBlueprintResources/StandardMacros.IsValid` (`self.ControlledHuman`)
      (:`Is Valid`
        (`/Game/ExampleContent/VR_World_Interaction/Blueprints/Components/BPC_WorldInteractor.PickupReleased` _bpc_worldinteractor_l)
        (`/Game/ExampleContent/VR_World_Interaction/Blueprints/Components/BPC_WorldInteractor.DragStop` _bpc_worldinteractor_l))
      (:`Is Not Valid`
        _))
    (`/Game/VirtualRealityBP/Blueprints/BP_MotionController.ReleaseActor` _lefthand)))

(event `InputAction|GrabRight`
  (params (Key :type "Key Structure"))
  (bind _righthand (`self.RightHand`))
  (bind _bpc_worldinteractor_r (`/Game/Blueprints/Humans/BaseHuman.BPC_WorldInteractor_R` (`self.ControlledHuman`)))
  (:`Pressed`
    (`/Engine/EditorBlueprintResources/StandardMacros.IsValid` (`self.ControlledHuman`)
      (:`Is Valid`
        (`/Game/ExampleContent/VR_World_Interaction/Blueprints/Components/BPC_WorldInteractor.PickupPressed` _bpc_worldinteractor_r)
        (`/Game/ExampleContent/VR_World_Interaction/Blueprints/Components/BPC_WorldInteractor.DragStart` _bpc_worldinteractor_r))
      (:`Is Not Valid`
        _))
    (`/Game/VirtualRealityBP/Blueprints/BP_MotionController.GrabActor` _righthand))
  (:`Released`
    (`/Engine/EditorBlueprintResources/StandardMacros.IsValid` (`self.ControlledHuman`)
      (:`Is Valid`
        (`/Game/ExampleContent/VR_World_Interaction/Blueprints/Components/BPC_WorldInteractor.PickupReleased` _bpc_worldinteractor_r)
        (`/Game/ExampleContent/VR_World_Interaction/Blueprints/Components/BPC_WorldInteractor.DragStop` _bpc_worldinteractor_r))
      (:`Is Not Valid`
        _))
    (`/Game/VirtualRealityBP/Blueprints/BP_MotionController.ReleaseActor` _righthand)))

(fn `CheckVehicleToDrive`
  (returns (`Hit Actor` :type "Actor Object Reference") (IsVehicleNear :type Boolean))
  (bind _returnvalue (`GameplayStatics.GetPlayerCameraManager` 0))
  (bind _returnvalue_2 (`self.K2_GetActorLocation` _returnvalue))
  (bind (_outhit _returnvalue_3) (`KismetSystemLibrary.LineTraceSingle` _returnvalue_2 (+ _returnvalue_2 (* (`self.GetActorForwardVector` _returnvalue) (`self.InteractionDistance`))) "TraceTypeQuery1" false (`|MakeArray` (`self.K2_GetPawn`) :!type "Actor Object Reference")))
  (return (`.HitActor` (`GameplayStatics.BreakHitResult` _outhit)) _returnvalue_3))

(fn `EnterVehicle`
  (params (ActorToUse :type "Actor Object Reference"))
  (bind _lefthand (`self.LeftHand`))
  (bind _righthand (`self.RightHand`))
  (bind _asbase_vehicle (cast `/Game/Blueprints/Vehicles/BaseVehicle` ActorToUse))
  (`self.UnPossess`)
  (`/Engine/EditorBlueprintResources/StandardMacros.IsValid` _lefthand
    (:`Is Valid`
      (`self.K2_DestroyActor` _lefthand)
      (`/Engine/EditorBlueprintResources/StandardMacros.IsValid` _righthand
        (:`Is Valid`
          (`self.K2_DestroyActor` _righthand))
        (:`Is Not Valid`
          _)))
    (:`Is Not Valid`
      _))
  (`self.Possess` _asbase_vehicle)
  (set `self.ControllingVehicle` true)
  (set `self.ControllingHuman` false)
  (`self.K2_DestroyActor` (`self.ControlledHuman`))
  (`self.K2_DestroyActor`))

(fn `LeaveAndEnterAircraft`)

(fn `LeaveVehicle`
  (bind _controlledvehicle (`self.ControlledVehicle`))
  (bind _lefthand (`self.LeftHand`))
  (bind _righthand (`self.RightHand`))
  (bind (_returnvalue_x _returnvalue_y _returnvalue_z) (`KismetMathLibrary.BreakVector` (+ (`self.K2_GetActorLocation` _controlledvehicle) (* (`self.GetActorRightVector` _controlledvehicle) (* (`.SphereRadius` (`KismetSystemLibrary.GetComponentBounds` (`WheeledVehicle.Mesh` _controlledvehicle))) -1.0)))))
  (`/Engine/EditorBlueprintResources/StandardMacros.IsValid` _lefthand
    (:`Is Valid`
      (`self.K2_DestroyActor` _lefthand)
      (`/Engine/EditorBlueprintResources/StandardMacros.IsValid` _righthand
        (:`Is Valid`
          (`self.K2_DestroyActor` _righthand))
        (:`Is Not Valid`
          _)))
    (:`Is Not Valid`
      _))
  (bind _returnvalue (`|SpawnActorFromClass` "/Game/Blueprints/Humans/Human_PlayerPawn.Human_PlayerPawn_C" (`KismetMathLibrary.MakeTransform` (`KismetMathLibrary.MakeVector` (+ _returnvalue_x 100.0) _returnvalue_y (+ _returnvalue_z 100.0)) (`self.K2_GetActorRotation` _controlledvehicle)) "AdjustIfPossibleButAlwaysSpawn" "OverrideRootScale" null null))
  (`self.Possess` _returnvalue)
  (set `self.ControlledHuman` _returnvalue)
  (set `self.ControllingVehicle` false)
  (set `self.ControllingHuman` true))

(fn `SetUpVR`
  (`HeadMountedDisplayFunctionLibrary.ResetOrientationAndPosition` 0.0))

(fn `UserConstructionScript`)