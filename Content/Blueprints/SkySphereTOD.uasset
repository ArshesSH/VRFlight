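; Sky sphere Blueprint that runs a day/night cycle and switches city meshes to emissive materials at night.
; Tick advances the hour by configurable day length, rotates the directional light and updates the sky's sun direction; construction applies the same sun angle.
; BeginPlay groups static mesh actors by material-name substrings.
; While time updates, every tick checks the night window and reapplies each group's normal or emissive slot-0 material.
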(event `self.ReceiveBeginPlay`
  (bind _output_get (set `self.OneDay` (* (`self.DayLengthInMinutes`) 60.0)))
  (set `self.OneHour` (/ _output_get 24.0))
  (`self.GetAllMeshesWithEmissiveTexture`))

(event `self.ReceiveTick`
  (params (DeltaSeconds :type "Float (single-precision)"))
  (bind (_returnvalue_roll _returnvalue_pitch _returnvalue_yaw) (`KismetMathLibrary.BreakRotator` (`self.K2_GetActorRotation`)))
  (bind _directional_light_actor (`self.Directional light actor`))
  (bind _returnvalue (+ (`self.Hour`) (/ DeltaSeconds (`self.OneHour`))))
  (if (`self.TimeUpdates`)
    (`self.CheckTime`)
    (if (>= _returnvalue 24.0)
      (set `self.Hour` 0.0)
      (else
        (set `self.Hour` _returnvalue)))
    (bind _output_get (set `self.SunAngle` (+ (* (/ (`self.Hour`) 6.0) 90.0) 90.0)))
    (`/Engine/EditorBlueprintResources/StandardMacros.IsValid` _directional_light_actor
      (:`Is Valid`
        (`self.K2_SetActorRotation` _directional_light_actor (`KismetMathLibrary.MakeRotator` 0.0 _output_get _returnvalue_yaw) false)
        (`self.UpdateSunDirection`)))))

(fn `CheckTime`
  (bind _hour (`self.Hour`))
  (if (`self.NightTime`)
    (set `self.NightTime` (not (`KismetMathLibrary.InRange_FloatFloat` (`self.Hour`) 6.0 20.0)))
    (else
      (set `self.NightTime` (or (`KismetMathLibrary.InRange_FloatFloat` _hour 0.0 6.0) (`KismetMathLibrary.InRange_FloatFloat` _hour 20.0 24.0)))))
  (`self.UpdateMeshesMaterials`))

(fn `GetAllMeshesWithEmissiveTexture`
  (`KismetArrayLibrary.Array_Clear` (`self.MeshesWithTexture01A`))
  (bind _outactors (`GameplayStatics.GetAllActorsOfClass` "/Script/Engine.StaticMeshActor"))
  (for _array_element _outactors
    (bind _returnvalue (`KismetSystemLibrary.GetDisplayName` (`PrimitiveComponent.GetMaterial` (`StaticMeshActor.StaticMeshComponent` _array_element) 0)))
    (if (`KismetStringLibrary.Contains` _returnvalue "_A")
      (if (`KismetStringLibrary.Contains` _returnvalue "01")
        (`KismetArrayLibrary.Array_AddUnique` (`self.MeshesWithTexture01A`) _array_element)
        (elif (`KismetStringLibrary.Contains` _returnvalue "02")
          (`KismetArrayLibrary.Array_AddUnique` (`self.MeshesWitheTexture02A`) _array_element)
          (elif (`KismetStringLibrary.Contains` _returnvalue "03")
            (`KismetArrayLibrary.Array_AddUnique` (`self.MeshesWitheTexture03A`) _array_element)
            (elif (`KismetStringLibrary.Contains` _returnvalue "04")
              (`KismetArrayLibrary.Array_AddUnique` (`self.MeshesWitheTexture04A`) _array_element))))))))

(fn `UpdateMeshArrayMaterial`
  (params (InputArray :type "Array of StaticMeshActor Object Reference") (MaterialToUse :type "MaterialInterface Object Reference"))
  (for _array_element InputArray
    (`PrimitiveComponent.SetMaterial` (`StaticMeshActor.StaticMeshComponent` _array_element) 0 MaterialToUse)))

(fn `UpdateMeshesMaterials`
  (bind _mesheswithtexture01a (`self.MeshesWithTexture01A`))
  (bind _mesheswithetexture02a (`self.MeshesWitheTexture02A`))
  (bind _mesheswithetexture03a (`self.MeshesWitheTexture03A`))
  (bind _mesheswithetexture04a (`self.MeshesWitheTexture04A`))
  (if (`self.NightTime`)
    (`self.UpdateMeshArrayMaterial` _mesheswithtexture01a "/Game/PolygonCity/Materials/Mat_PolygonCity_Texture_01_A_Emissive.Mat_PolygonCity_Texture_01_A_Emissive")
    (`self.UpdateMeshArrayMaterial` _mesheswithetexture02a "/Game/PolygonCity/Materials/Mat_PolygonCity_Texture_02_A_Emissive.Mat_PolygonCity_Texture_02_A_Emissive")
    (`self.UpdateMeshArrayMaterial` _mesheswithetexture03a "/Game/PolygonCity/Materials/Mat_PolygonCity_Texture_03_A_Emissive.Mat_PolygonCity_Texture_03_A_Emissive")
    (`self.UpdateMeshArrayMaterial` _mesheswithetexture04a "/Game/PolygonCity/Materials/Mat_PolygonCity_Texture_04_A_Emissive.Mat_PolygonCity_Texture_04_A_Emissive")
    (else
      (`self.UpdateMeshArrayMaterial` _mesheswithtexture01a "/Game/PolygonCity/Materials/Mat_PolygonCity_Texture_01_A.Mat_PolygonCity_Texture_01_A")
      (`self.UpdateMeshArrayMaterial` _mesheswithetexture02a "/Game/PolygonCity/Materials/Mat_PolygonCity_Texture_02_A.Mat_PolygonCity_Texture_02_A")
      (`self.UpdateMeshArrayMaterial` _mesheswithetexture03a "/Game/PolygonCity/Materials/Mat_PolygonCity_Texture_03_A.Mat_PolygonCity_Texture_03_A")
      (`self.UpdateMeshArrayMaterial` _mesheswithetexture04a "/Game/PolygonCity/Materials/Mat_PolygonCity_Texture_04_A.Mat_PolygonCity_Texture_04_A"))))

(fn `UserConstructionScript`
  (bind (_returnvalue_roll _returnvalue_pitch _returnvalue_yaw) (`KismetMathLibrary.BreakRotator` (`self.K2_GetActorRotation`)))
  (bind _directional_light_actor (`self.Directional light actor`))
  (`parent.UserConstructionScript`)
  (bind _output_get (set `self.SunAngle` (+ (* (/ (`self.Hour`) 6.0) 90.0) 90.0)))
  (`/Engine/EditorBlueprintResources/StandardMacros.IsValid` _directional_light_actor
    (:`Is Valid`
      (`self.K2_SetActorRotation` _directional_light_actor (`KismetMathLibrary.MakeRotator` 0.0 _output_get _returnvalue_yaw) false)
      (`self.UpdateSunDirection`))))