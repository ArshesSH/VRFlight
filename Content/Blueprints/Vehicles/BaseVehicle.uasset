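; Base vehicle pawn with zoomable third-person and first-person cameras, a randomly chosen mesh material, and VR support.
; On possession it attaches a flight stick, and for a human controller with an active headset also spawns both motion controllers and registers them as its hands.
; A gate, open only for human control, smooths spring arm length toward the zoom target on Tick.
; Zooming fully in switches to the first-person camera; zooming out switches back.
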(event `self.ReceiveBeginPlay`
  (set `self.DesiredTargetArmLength` (`SpringArmComponent.TargetArmLength` (`self.SpringArm`))))

(event `self.ReceiveTick`
  (params (DeltaSeconds :type "Float (single-precision)"))
  (bind _springarm (`self.SpringArm`))
  (`/Engine/EditorBlueprintResources/StandardMacros.Gate` true :!label _label
    (:`Exit`
      (set `SpringArmComponent.TargetArmLength` (`KismetMathLibrary.FInterpTo` (`SpringArmComponent.TargetArmLength` _springarm) (`self.DesiredTargetArmLength`) (`GameplayStatics.GetWorldDeltaSeconds`) 3.0) _springarm))))

(event `self.ReceivePossessed`
  (params (NewController :type "Controller Object Reference"))
  (`KismetSystemLibrary.Delay` 0.2)
  (`self.SetStick`)
  (cast `/Game/Blueprints/Controllers/PC_HumanController` NewController
    (:`then`
      (if (`HeadMountedDisplayFunctionLibrary.IsHeadMountedDisplayEnabled`)
        (`self.SetUpVR`)
        (goto _label :!via `Open`)
        (else
          (goto _label :!via `Open`))))
    (:`CastFailed`
      (goto _label :!via `Close`))))

(fn `SetRandomMaterial`
  (bind _materialtouse (`self.MaterialToUse`))
  (`PrimitiveComponent.SetMaterial` (`self.Mesh`) 0 (`|GetArrayItem` _materialtouse (`KismetMathLibrary.RandomIntegerInRange` 0 (`KismetArrayLibrary.Array_LastIndex` _materialtouse)))))

(fn `SetStick`
  (bind _returnvalue (`|SpawnActorFromClass` "/Game/Blueprints/Vehicles/BP_FlightStick_Fix.BP_FlightStick_Fix_C" (`KismetMathLibrary.MakeTransform` (0.0 0.0 0.0)) "Undefined" "OverrideRootScale" self null))
  (`SceneComponent.K2_AttachToComponent` (`Actor.RootComponent` _returnvalue) (`self.StickPosition`) "None" "KeepRelative" "KeepRelative" "KeepRelative" false))

(fn `SetUpVR`
  (bind _returnvalue (`KismetMathLibrary.MakeTransform` (0.0 0.0 0.0)))
  (bind _returnvalue_2 (`self.GetController`))
  (`|ExecutionSequence`
    (:`then_0`
      (bind _returnvalue_3 (`|SpawnActorFromClass` "/Game/VirtualRealityBP/Blueprints/BP_MotionController.BP_MotionController_C" _returnvalue "Undefined" "OverrideRootScale" _returnvalue_2 "Left" null))
      (`self.K2_AttachToComponent` _returnvalue_3 (`self.Scene`) "None" "SnapToTarget" "SnapToTarget" "SnapToTarget" false)
      (bind _aspc_human_controller (cast `/Game/Blueprints/Controllers/PC_HumanController` (`self.GetController`)))
      (set `/Game/Blueprints/Controllers/PC_HumanController.LeftHand` _returnvalue_3 _aspc_human_controller))
    (:`then_1`
      (bind _returnvalue_4 (`|SpawnActorFromClass` "/Game/VirtualRealityBP/Blueprints/BP_MotionController.BP_MotionController_C" _returnvalue "Undefined" "OverrideRootScale" _returnvalue_2 "Right" null))
      (`self.K2_AttachToComponent` _returnvalue_4 (`self.Scene`) "None" "SnapToTarget" "SnapToTarget" "SnapToTarget" false)
      (bind _aspc_human_controller_2 (cast `/Game/Blueprints/Controllers/PC_HumanController` (`self.GetController`)))
      (set `/Game/Blueprints/Controllers/PC_HumanController.RightHand` _returnvalue_4 _aspc_human_controller_2))))

(fn `UserConstructionScript`
  (`self.SetRandomMaterial`))

(fn `ZoomIn`
  (if (<= (`self.DesiredTargetArmLength`) 300.0)
    (`ActorComponent.Deactivate` (`self.TPVCamera`))
    (`ActorComponent.SetActive` (`self.FPVCamera`) true true)
    (else
      (set `self.DesiredTargetArmLength` (`KismetMathLibrary.FClamp` (- (`self.DesiredTargetArmLength`) 20.0) 275.0 1000.0)))))

(fn `ZoomOut`
  (bind _tpvcamera (`self.TPVCamera`))
  (if (`ActorComponent.IsActive` _tpvcamera)
    (set `self.DesiredTargetArmLength` (`KismetMathLibrary.FClamp` (+ (`self.DesiredTargetArmLength`) 20.0) 0.0 1000.0))
    (else
      (`ActorComponent.Deactivate` (`self.FPVCamera`))
      (`ActorComponent.SetActive` _tpvcamera true true))))