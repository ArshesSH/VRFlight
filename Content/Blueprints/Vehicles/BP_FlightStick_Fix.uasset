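; Grabbable flight stick actor for a vehicle that tilts and twists with the hand holding it, then recenters on release.
; Pickup attaches a proxy ball to the grabber; Tick turns its offset from a reference arrow, plus its yaw, into clamped stick rotation filtered by CheckDeadzone.
; Drop detaches the ball, and a timeline eases the stick to neutral while returning the ball to the arrow.
; Other interaction functions are empty stubs.
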(event `/Game/VirtualRealityBP/Blueprints/PickupActorInterface.Pickup`
  (params (AttachTo :type "SceneComponent Object Reference"))
  (set `self.IsGrabbed` true)
  (`SceneComponent.K2_AttachToComponent` (`self.StickBallHand`) AttachTo "None" "KeepWorld" "KeepWorld" "KeepWorld" false)
  (`SceneComponent.ToggleVisibility` (`self.StickBallHand`) false))

(event `self.ReceiveTick`
  (params (DeltaSeconds :type "Float (single-precision)"))
  (bind _stick (`self.Stick`))
  (bind (_returnvalue_roll _returnvalue_pitch) (`KismetMathLibrary.BreakRotator` (`SceneComponent.K2_GetComponentRotation` _stick)))
  (bind (_returnvalue_roll_2 _returnvalue_pitch_2 _returnvalue_yaw) (`KismetMathLibrary.BreakRotator` (`SceneComponent.K2_GetComponentRotation` (`self.StickBallHand`))))
  (bind _relativelocation (`SceneComponent.RelativeLocation` (`self.StickBallHand`)))
  (bind (_returnvalue_x _returnvalue_y) (`KismetMathLibrary.BreakVector` (- (`SceneComponent.K2_GetComponentLocation` (`self.StickBallHand`)) (`SceneComponent.K2_GetComponentLocation` (`self.Arrow`)))))
  (bind _returnvalue_x_2 (`KismetMathLibrary.BreakVector` (- (`SceneComponent.RelativeLocation` (`self.Arrow`)) _relativelocation)))
  (if (`self.IsGrabbed`)
    (bind (_axisx_output _axisy_output _axisz_output) (`self.CheckDeadzone` (`KismetMathLibrary.FClamp` (+ _returnvalue_pitch _returnvalue_x_2) -25.0 25.0) (`KismetMathLibrary.FClamp` (+ _returnvalue_roll _returnvalue_y) -25.0 25.0) (`KismetMathLibrary.ClampAngle` _returnvalue_yaw -25.0 25.0) 2.0))
    (`SceneComponent.K2_SetWorldRotation` _stick (`KismetMathLibrary.MakeRotator` _axisy_output _axisx_output _axisz_output) false false)
    (`KismetSystemLibrary.PrintString` (`KismetStringLibrary.Conv_VectorToString` _relativelocation))))

(event `/Game/VirtualRealityBP/Blueprints/PickupActorInterface.Drop`
  (bind _arrow (`self.Arrow`))
  (set `self.IsGrabbed` false)
  (`SceneComponent.ToggleVisibility` (`self.StickBallHand`) false)
  (`SceneComponent.K2_DetachFromComponent` (`self.StickBallHand`) "KeepWorld" "KeepWorld" "KeepWorld" true)
  (set `self.ResettingRotation` true)
  (set `self.InterpStickRotation` (`SceneComponent.RelativeRotation` (`self.Stick`)))
  (bind (_direction _alpha) (`Timeline|ResetRotationTimeline` :!via `PlayFromStart`)
    (:`Update`
      (if (`self.IsGrabbed`)
        (set `self.ResettingRotation` false :!label _label)
        (else
          (`SceneComponent.K2_SetRelativeRotation` (`self.Stick`) (`KismetMathLibrary.RLerp` (`self.InterpStickRotation`) (struct) _alpha) false false)
          (`SceneComponent.K2_SetRelativeLocationAndRotation` (`self.StickBallHand`) (`SceneComponent.K2_GetComponentLocation` _arrow) (`SceneComponent.K2_GetComponentRotation` _arrow) false false))))
    (:`Finished`
      (goto _label))))

(fn `CheckDeadzone`
  (params (AxisX_Input :type "Float (double-precision)") (AxisY_Input :type "Float (double-precision)") (AxisZ_Input :type "Float (double-precision)") (DeadzoneValue :type "Float (double-precision)"))
  (returns (AxisX_Output :type "Float (double-precision)") (AxisY_Output :type "Float (double-precision)") (AxisZ_Output :type "Float (double-precision)"))
  (locals (Axis_Z :type "Float (double-precision)"))
  (bind _returnvalue (* DeadzoneValue 2.0))
  (bind _output_get (set `local.Axis_Z` AxisZ_Input))
  (if (`KismetMathLibrary.InRange_FloatFloat` _output_get (- 0.0 _returnvalue) _returnvalue)
    (set `local.Axis_Z` 0.0))
  (if (and (`KismetMathLibrary.InRange_FloatFloat` AxisX_Input (- 0.0 DeadzoneValue) DeadzoneValue) (`KismetMathLibrary.InRange_FloatFloat` AxisY_Input (- 0.0 DeadzoneValue) DeadzoneValue))
    (return 0.0 0.0 (`local.Axis_Z`))
    (else
      (return AxisX_Input AxisY_Input (`local.Axis_Z`)))))

(fn `GetAnimSequence`
  (params (Hand :type "EControllerHand Enum" :default "Left"))
  (returns (AnimSequence :type "AnimSequence Object Reference"))
  (return null))

(fn `GetClosestComponentData`
  (params (Interactor :type "/Game/ExampleContent/VR_World_Interaction/Blueprints/Components/BPC_WorldInteractor Object Reference"))
  (returns (Point :type "Vector Structure") (Priority :type Integer) (Component :type "SceneComponent Object Reference"))
  (return (0.0 0.0 0.0) 0 null))

(fn `GetPickupComponent`
  (returns (PickupComponent :type "/Game/Hands/BPC_PickupObject Object Reference"))
  (return null))

(fn `OnDrag`
  (params (Interactor :type "/Game/ExampleContent/VR_World_Interaction/Blueprints/Components/BPC_WorldInteractor Object Reference"))
  (returns (Return :type Boolean))
  (return false))

(fn `OnDragStart`
  (params (Interactor :type "/Game/ExampleContent/VR_World_Interaction/Blueprints/Components/BPC_WorldInteractor Object Reference"))
  (returns (Return :type Boolean))
  (return false))

(fn `OnDragStop`
  (params (Interactor :type "/Game/ExampleContent/VR_World_Interaction/Blueprints/Components/BPC_WorldInteractor Object Reference"))
  (returns (Return :type Boolean))
  (return false))

(fn `OnHover`
  (params (Interactor :type "/Game/ExampleContent/VR_World_Interaction/Blueprints/Components/BPC_WorldInteractor Object Reference"))
  (returns (Return :type Boolean))
  (return false))

(fn `OnHoveredComponentChanged`
  (params (Interactor :type "/Game/ExampleContent/VR_World_Interaction/Blueprints/Components/BPC_WorldInteractor Object Reference") (OldComponent :type "SceneComponent Object Reference") (NewComponent :type "SceneComponent Object Reference"))
  (returns (Return :type Boolean))
  (return false))

(fn `OnPickupPressed`
  (params (Interactor :type "/Game/ExampleContent/VR_World_Interaction/Blueprints/Components/BPC_WorldInteractor Object Reference"))
  (returns (Return :type Boolean))
  (return false))

(fn `OnPickupReleased`
  (params (Interactor :type "/Game/ExampleContent/VR_World_Interaction/Blueprints/Components/BPC_WorldInteractor Object Reference"))
  (returns (Return :type Boolean))
  (return false))

(fn `OnUnhover`
  (params (Interactor :type "/Game/ExampleContent/VR_World_Interaction/Blueprints/Components/BPC_WorldInteractor Object Reference"))
  (returns (Return :type Boolean))
  (return false))

(fn `OnUsePressed`
  (params (Interactor :type "/Game/ExampleContent/VR_World_Interaction/Blueprints/Components/BPC_WorldInteractor Object Reference"))
  (returns (Return :type Boolean))
  (return false))

(fn `OnUseReleased`
  (params (Interactor :type "/Game/ExampleContent/VR_World_Interaction/Blueprints/Components/BPC_WorldInteractor Object Reference"))
  (returns (Return :type Boolean))
  (return false))

(fn `UserConstructionScript`)