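; BP_AoAIndexer is an angle-of-attack indexer for the player's F-16C, lighting High, Approch and Low indicators to show approach speed cues.
; On BeginPlay it casts the player pawn to BP_F-16C and caches its FlightModel.
; Each Tick it reads Alpha and toggles the three components' visibility across five bands, lighting adjacent pairs in the transitional bands.
; The slow-to-fast boolean state assignments are never executed.
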(event `self.ReceiveBeginPlay`
  (bind _asbp_f_16c (cast `/Game/untitled_category/untitled_asset/F-16C/BP_F-16C` (`GameplayStatics.GetPlayerPawn` 0)))
  (set `self.Flight Model` (`/Game/untitled_category/untitled_asset/F-16C/BP_F-16C.FlightModel` _asbp_f_16c)))

(event `self.ReceiveTick`
  (params (DeltaSeconds :type "Float (single-precision)"))
  (set `self.Alpha` (`.Alpha` (`easyFM.GetData` (`self.Flight Model`) "GDF_Imperial" false)))
  (if (> (`self.Alpha`) 9.3)
    (`SceneComponent.SetVisibility` (`self.High`) true false)
    (`SceneComponent.SetVisibility` (`self.Approch`) false false)
    (`SceneComponent.SetVisibility` (`self.Low`) false false)
    (elif (`KismetMathLibrary.InRange_FloatFloat` (`self.Alpha`) 8.8 9.3 false)
      (`SceneComponent.SetVisibility` (`self.High`) true false)
      (`SceneComponent.SetVisibility` (`self.Approch`) true false)
      (`SceneComponent.SetVisibility` (`self.Low`) false false)
      (elif (`KismetMathLibrary.InRange_FloatFloat` (`self.Alpha`) 7.4 8.8 false)
        (`SceneComponent.SetVisibility` (`self.High`) false false)
        (`SceneComponent.SetVisibility` (`self.Approch`) true false)
        (`SceneComponent.SetVisibility` (`self.Low`) false false)
        (elif (`KismetMathLibrary.InRange_FloatFloat` (`self.Alpha`) 6.9 7.4)
          (`SceneComponent.SetVisibility` (`self.High`) false false)
          (`SceneComponent.SetVisibility` (`self.Approch`) true false)
          (`SceneComponent.SetVisibility` (`self.Low`) true false)
          (elif (< (`self.Alpha`) 6.9)
            (`SceneComponent.SetVisibility` (`self.High`) false false)
            (`SceneComponent.SetVisibility` (`self.Approch`) false false)
            (`SceneComponent.SetVisibility` (`self.Low`) true false)))))))

(fn `UserConstructionScript`)