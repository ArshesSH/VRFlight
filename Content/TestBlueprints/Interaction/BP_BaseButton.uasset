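; BP_BaseButton is a physical push button pressed with the player pawn's right motion controller.
; On overlap it records start positions, then each Tick projects controller movement onto the button's up axis and sinks the button by that absolute, clamped distance.
; Reaching maximum travel calls FullyPressed, which only ends tracking and starts the return.
; Ending overlap does the same, and Tick eases the button back with VInterpTo.
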(event `self.Button .OnComponentBeginOverlap`
  (params (OverlappedComponent :type "PrimitiveComponent Object Reference") (OtherActor :type "Actor Object Reference") (OtherComp :type "PrimitiveComponent Object Reference") (OtherBodyIndex :type Integer) (bFromSweep :type Boolean) (SweepResult :type "HitResult Structure (by ref)"))
  (bind _ashuman_player_pawn_test (cast `/Game/TestBlueprints/Character/Human_PlayerPawn_TEST` OtherActor))
  (set `self.TrackingMotionController` (`/Game/TestBlueprints/Character/BaseHuman_TEST.MotionController_R` _ashuman_player_pawn_test))
  (set `self.bIsTracking` true)
  (set `self.MotionControllerInitialLocation` (`SceneComponent.K2_GetComponentLocation` (`self.TrackingMotionController`)))
  (set `self.ButtonInitialLocation` (`SceneComponent.K2_GetComponentLocation` (`self.Button `))))

(event `self.ReceiveTick`
  (params (DeltaSeconds :type "Float (single-precision)"))
  (bind _button_ (`self.Button `))
  (if (`self.bIsTracking`)
    (set `self.CurrentTravel` (`KismetMathLibrary.FClamp` (`KismetMathLibrary.Abs` (`KismetMathLibrary.VSize` (`KismetMathLibrary.ProjectVectorOnToVector` (- (`SceneComponent.K2_GetComponentLocation` (`self.TrackingMotionController`)) (`self.MotionControllerInitialLocation`)) (`SceneComponent.GetUpVector` (`self.Button `))))) 0.0 (`self.MaximumTravel`)))
    (bind _output_get (set `self.ButtonCurrentLocation` (- (`self.ButtonInitialLocation`) (* (`SceneComponent.GetUpVector` _button_) (`self.CurrentTravel`)))))
    (`SceneComponent.K2_SetWorldLocation` _button_ _output_get false false)
    (if (>= (`self.CurrentTravel`) (`self.MaximumTravel`))
      (`self.Fully Pressed`))
    (elif (`self.bIsReturning`)
      (bind _output_get_2 (set `self.ButtonCurrentLocation` (`KismetMathLibrary.VInterpTo` (`self.ButtonCurrentLocation`) (`self.ButtonInitialLocation`) (`GameplayStatics.GetWorldDeltaSeconds`) 2.0)))
      (`SceneComponent.K2_SetWorldLocation` (`self.Button `) _output_get_2 false false)
      (if (`KismetMathLibrary.EqualExactly_VectorVector` (`self.ButtonCurrentLocation`) (`self.ButtonInitialLocation`))
        (set `self.bIsReturning` false)))))

(event `Fully Pressed`
  (set `self.bIsTracking` false)
  (set `self.bIsReturning` true))

(event `self.Button .OnComponentEndOverlap`
  (params (OverlappedComponent :type "PrimitiveComponent Object Reference") (OtherActor :type "Actor Object Reference") (OtherComp :type "PrimitiveComponent Object Reference") (OtherBodyIndex :type Integer))
  (bind _ashuman_player_pawn_test (cast `/Game/TestBlueprints/Character/Human_PlayerPawn_TEST` OtherActor))
  (if (== (`/Game/TestBlueprints/Character/BaseHuman_TEST.MotionController_R` _ashuman_player_pawn_test) (`self.TrackingMotionController`))
    (set `self.bIsTracking` false)
    (set `self.bIsReturning` true)))

(fn `UserConstructionScript`)