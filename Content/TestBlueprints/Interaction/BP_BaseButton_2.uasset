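; BP_BaseButton_2 is a test interactive button that animates a press when a BP_Hand overlaps its Button component.
; Two chained MoveComponentTo calls lower and raise it, guarded by IsPressed.
; IsPressed is set before the hand cast, so any non-hand overlap leaves it locked.
; Disconnected logic remains for tracking motion-controller travel along the button's up vector and interpolating it back after a full press.
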(event `self.Button .OnComponentBeginOverlap`
  (params (OverlappedComponent :type "PrimitiveComponent Object Reference") (OtherActor :type "Actor Object Reference") (OtherComp :type "PrimitiveComponent Object Reference") (OtherBodyIndex :type Integer) (bFromSweep :type Boolean) (SweepResult :type "HitResult Structure (by ref)"))
  (bind _button_ (`self.Button `))
  (bind _button__2 (`self.Button `))
  (bind (_returnvalue_location _returnvalue_rotation) (`KismetMathLibrary.BreakTransform` (`SceneComponent.GetRelativeTransform` _button_)))
  (bind (_returnvalue_location_2 _returnvalue_rotation_2) (`KismetMathLibrary.BreakTransform` (`SceneComponent.GetRelativeTransform` _button__2)))
  (if (not (`self.bIsPressed`))
    (set `self.bIsPressed` true)
    (cast `/Game/Hands/BP_Hand` OtherActor)
    (`KismetSystemLibrary.MoveComponentTo` _button__2 (- _returnvalue_location_2 (0.0 0.0 15.0)) _returnvalue_rotation_2 false false 0.25)
    (`KismetSystemLibrary.MoveComponentTo` _button_ (- _returnvalue_location (0.0 0.0 -15.0)) _returnvalue_rotation false false 0.25)
    (set `self.bIsPressed` false)))

(event `self.ReceiveTick`
  (params (DeltaSeconds :type "Float (single-precision)")))

(event `Fully Pressed`
  (set `self.bIsTracking` false)
  (set `self.bIsReturning` true))

(fn `UserConstructionScript`)