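; BP_MainPowerSwitch is an instrument switch that turns the F16's main power on and off.
; On BeginPlay it runs the parent setup, tilts SpinPoint to the down position and flags Down as the active input.
; SwitchMiddle calls MainPowerOn on the F16 and SwitchDown calls MainPowerOFF, with no handling for an up position in this Blueprint.
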(event `self.ReceiveBeginPlay`
  (`parent.ReceiveBeginPlay`)
  (`SceneComponent.K2_SetRelativeRotation` (`self.SpinPoint`) (`KismetMathLibrary.MakeRotator` 25.0) false false)
  (set `self.bInputUp` false)
  (set `self.bInputDown` true)
  (set `self.bInputMiddle` false))

(event `self.SwitchMiddle`
  (`/Game/Asset/F-16C/BP_F-16C.MainPowerOn` (`self.F-16`)))

(event `self.SwitchDown`
  (`/Game/Asset/F-16C/BP_F-16C.MainPowerOFF` (`self.F-16`)))

(fn `UserConstructionScript`
  (`parent.UserConstructionScript`))