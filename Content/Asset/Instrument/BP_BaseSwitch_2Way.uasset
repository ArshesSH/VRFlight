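; Base VR-grabbable two-way switch whose stick rolls between up and down positions.
; While held, the hidden control ball follows the hand, and a gated Tick turns its local Y offset into clamped roll, snapping near either end and latching up/down input.
; On release the ball reattaches to the stick; if ReturnPos is set, a timeline eases the stick to neutral, calling empty SwitchUp/SwitchDown stubs on updates.
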(event `/Game/VirtualRealityBP/Blueprints/PickupActorInterface.Pickup`
  (params (AttachTo :type "SceneComponent Object Reference"))
  (bind _output_get (set `self.Hand` AttachTo))
  (`SceneComponent.ToggleVisibility` (`self.ControlBall`) false)
  (set `self.bIsGrabbed` true)
  (`SceneComponent.K2_AttachToComponent` (`self.ControlBall`) _output_get "None" "KeepWorld" "KeepWorld" "KeepRelative" false) ; Attach Control Ball to VR Hand
  (`self.Start Tick`))

(event `/Game/VirtualRealityBP/Blueprints/PickupActorInterface.Drop`
  (bind _controlballpositon (`self.ControlBallPositon`))
  (`self.Stop Tick`)
  (set `self.Hand` null)
  (set `self.bIsGrabbed` false)
  (set `self.Interp Rotator` (`SceneComponent.RelativeRotation` (`self.SpinPoint`)))
  (`SceneComponent.ToggleVisibility` (`self.ControlBall`) false)
  (`SceneComponent.K2_DetachFromComponent` (`self.ControlBall`) "KeepWorld" "KeepWorld" "KeepWorld" false) ; Detach Control Ball from VR Hand
  (`SceneComponent.K2_AttachToComponent` (`self.ControlBall`) (`self.ControlBallPositon`) "None" "KeepRelative" "KeepRelative" "KeepRelative" false) ; Attach Control Ball to Stick Ball Position.\nReset Control Ball's Position
  (`SceneComponent.K2_SetWorldLocationAndRotation` (`self.ControlBall`) (`SceneComponent.K2_GetComponentLocation` _controlballpositon) (`SceneComponent.K2_GetComponentRotation` _controlballpositon) false false)
  (if (`self.bReturnPos`)
    (bind (_direction `_새_트랙_0`) (`Timeline|타임라인_0` :!via `PlayFromStart`)
      (:`Update`
        (if (not (`self.bIsGrabbed`))
          (`SceneComponent.K2_SetRelativeRotation` (`self.SpinPoint`) (`KismetMathLibrary.RLerp` (`self.Interp Rotator`) (struct) `_새_트랙_0`) false false)
          (if (`self.bInputUp`)
            (`self.SwitchUp`)
            (elif (`self.bInputDown`)
              (`self.SwitchDown`))))))))

(event `self.ReceiveTick`
  (params (DeltaSeconds :type "Float (single-precision)"))
  (`/Engine/EditorBlueprintResources/StandardMacros.Gate` true :!label _label
    (:`Exit`
      (bind _output_get (set `self.YAxis` (`KismetMathLibrary.FClamp` (/ (.y (.location (`KismetMathLibrary.ConvertTransformToRelative` (`SceneComponent.K2_GetComponentToWorld` (`self.ControlBall`)) (`SceneComponent.K2_GetComponentToWorld` (`self.Scene`))))) -5.0) -25.0 25.0)))
      (`SceneComponent.K2_SetRelativeRotation` (`self.SpinPoint`) (`KismetMathLibrary.MakeRotator` _output_get) false false)
      (if (`KismetMathLibrary.InRange_FloatFloat` (`self.YAxis`) 15.0 25.0)
        (`SceneComponent.K2_SetRelativeRotation` (`self.SpinPoint`) (`KismetMathLibrary.MakeRotator` 25.0) false false)
        (set `self.bInputUp` false)
        (set `self.bInputDown` true)
        (elif (`KismetMathLibrary.InRange_FloatFloat` (`self.YAxis`) -25.0 -15.0)
          (`SceneComponent.K2_SetRelativeRotation` (`self.SpinPoint`) (`KismetMathLibrary.MakeRotator` -25.0) false false)
          (set `self.bInputUp` true)
          (set `self.bInputDown` false))))))

(event `Start Tick`
  (goto _label :!via `Open`))

(event `Stop Tick`
  (goto _label :!via `Close`))

(fn `GetAnimSequence`
  (params (Hand :type "EControllerHand Enum" :default "Left"))
  (returns (AnimSequence :type "AnimSequence Object Reference"))
  (return null))

(fn `GetPickupComponent`
  (returns (PickupComponent :type "/Game/Hands/BPC_PickupObject Object Reference"))
  (return null))

(fn `SwitchDown`)

(fn `SwitchUp`)

(fn `UserConstructionScript`)