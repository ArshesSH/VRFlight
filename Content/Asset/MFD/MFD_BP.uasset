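; MFD Blueprint for an aircraft-style multifunction display that switches between Menu, Blank, TFR, SMS and HSD pages.
; OpenMenu shows the menu widget and hides the other page widgets along with the TFR Line and HSD Plane components.
; Page toggles and flag-driven updates that rotate Plane from root yaw and move Line to root height are unconnected, so only OpenMenu does anything.
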(event `self.ReceiveBeginPlay`)

(event `self.ReceiveTick`
  (params (DeltaSeconds :type "Float (single-precision)")))

(event `OpenMenu`
  ;[1 1 1] Menu
  (`SceneComponent.SetVisibility` (`self.Menu_Widget`) true false)
  (`SceneComponent.SetVisibility` (`self.Blank_Widget`) false false)
  (`SceneComponent.SetVisibility` (`self.TFR_Widget`) false false)
  (`SceneComponent.SetVisibility` (`self.Line`) false false)
  (`SceneComponent.SetVisibility` (`self.SMS_Widget`) false false)
  (`SceneComponent.SetVisibility` (`self.HSD_Widget`) false false)
  (`SceneComponent.SetVisibility` (`self.Plane`) false false))

(fn `UserConstructionScript`)