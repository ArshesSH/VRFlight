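; F-16C cockpit landing gear switch that a hand grabs and releases to flip between up and down.
; While held, a gated Tick shows ControlBall near the hand and flags a cancel when the hand strays too far.
; An uncancelled Drop toggles the state, turns the player jet's gear panel light on for down or off for up, and timeline-lerps SpinPoint's pitch.
; The construction script poses the lever from IsSwitchUp.
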(event `self.ReceiveBeginPlay`
  (bind _asbp_f_16c (cast `/Game/Asset/F-16C/BP_F-16C` (`GameplayStatics.GetPlayerPawn` 0)))
  (set `self.Landiggear Pannel` (`/Game/Asset/F-16C/BP_F-16C.LandiggearPannel` _asbp_f_16c)))

(event `/Game/VirtualRealityBP/Blueprints/PickupActorInterface.Pickup`
  (params (AttachTo :type "SceneComponent Object Reference"))
  (set `self.Hand` AttachTo)
  (`SceneComponent.SetVisibility` (`self.ControlBall`) true false)
  (`self.Start Tick`))

(event `/Game/VirtualRealityBP/Blueprints/PickupActorInterface.Drop`
  (bind _landiggear_pannel (`self.Landiggear Pannel`))
  (`self.Stop Tick`)
  (if (not (`self.bIsCancel`))
    (`SceneComponent.SetVisibility` (`self.ControlBall`) false false)
    (if (`self.bIsSwitchUp`)
      (set `self.DefaultPos` 30.0)
      (set `self.bIsSwitchUp` false)
      (`/Game/Asset/LandinggearPanel/BP_LandingearPanel.LightOn` _landiggear_pannel)
      (else
        (set `self.DefaultPos` -50.0)
        (set `self.bIsSwitchUp` true)
        (`/Game/Asset/LandinggearPanel/BP_LandingearPanel.LightOff` _landiggear_pannel)))
    (set `self.InterpRotator` (`SceneComponent.RelativeRotation` (`self.SpinPoint`)))
    (bind (_direction `_새_트랙_0`) (`Timeline|타임라인_0` :!via `PlayFromStart`)
      (:`Update`
        (`SceneComponent.K2_SetRelativeRotation` (`self.SpinPoint`) (`KismetMathLibrary.RLerp` (`self.InterpRotator`) (`KismetMathLibrary.MakeRotator` 0.0 (`self.DefaultPos`)) `_새_트랙_0`) false false)))))

(event `self.ReceiveTick`
  (params (DeltaSeconds :type "Float (single-precision)"))
  (`/Engine/EditorBlueprintResources/StandardMacros.Gate` true :!label _label
    (:`Exit`
      (bind _output_get (set `self.Distance` (`KismetMathLibrary.Vector_Distance` (`SceneComponent.K2_GetComponentLocation` (`self.Hand`)) (`SceneComponent.K2_GetComponentLocation` (`self.ControlBall`)))))
      (if (> _output_get 20.0)
        (set `self.bIsCancel` true)
        (`SceneComponent.SetVisibility` (`self.ControlBall`) false false)
        (else
          (set `self.bIsCancel` false)
          (`SceneComponent.SetVisibility` (`self.ControlBall`) true false))))))

(event `Start Tick`
  (goto _label :!via `Open`))

(event `Stop Tick`
  (goto _label :!via `Close`))

(fn `GetAnimSequence`
  (params (Hand :type "EControllerHand Enum" :default "Left"))
  (returns (AnimSequence :type "AnimSequence Object Reference"))
  (return null))

(fn `GetPickupComponent`
  (returns (PickupComponent :type "/Game/Hands/BPC_PickupObject Object Reference"))
  (return null))

(fn `UserConstructionScript`
  (if (`self.bIsSwitchUp`)
    (bind _output_get (set `self.DefaultPos` -50.0))
    (`SceneComponent.K2_SetRelativeRotation` (`self.SpinPoint`) (`KismetMathLibrary.MakeRotator` 0.0 _output_get) false false)
    (else
      (bind _output_get_2 (set `self.DefaultPos` 50.0))
      (`SceneComponent.K2_SetRelativeRotation` (`self.SpinPoint`) (`KismetMathLibrary.MakeRotator` 0.0 _output_get_2) false false))))