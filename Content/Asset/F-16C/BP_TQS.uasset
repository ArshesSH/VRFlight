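; VR-grabbable F-16C throttle lever (TQS) that outputs a clamped ThrottleValue from its angle.
; While grabbed, a gated Tick projects the hand onto the lever's travel axis and rotates SpinPoint within AngleMin/AngleMax.
; Hand roll twists HingePoint, which a timeline eases back on release as ControlBall returns to the stick.
; Idle, normal and afterburner range switching is present but not wired into the running graph.
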(event `self.ReceiveBeginPlay`
  ;[1 1 1] Set UPVector
  (set `self.InitialUpVector` (`SceneComponent.GetUpVector` (`self.SpinPoint`)))
  ;[1 1 1] Spin to Idle Angle
  (`SceneComponent.K2_SetWorldRotation` (`self.SpinPoint`) (`self.GetTQSRotationAtAngle` (`self.AngleIdleMin`)) false false)
  (set `self.bIsIdle` true))

(event `/Game/VirtualRealityBP/Blueprints/PickupActorInterface.Drop`
  (bind _controlpoint (`self.ControlPoint`))
  (bind _controlball (`self.ControlBall`))
  ;[1 1 1] Drop
  (`self.Stop Tracking`)
  (set `self.Hand` null)
  (set `self.bIsGrabbed` false)
  (`SceneComponent.K2_DetachFromComponent` _controlball "KeepWorld" "KeepWorld" "KeepWorld" false) ; Detach Control Ball from VR Hand
  (`SceneComponent.K2_AttachToComponent` _controlball (`self.ControlPoint`) "None" "KeepRelative" "KeepRelative" "KeepRelative" false) ; Attach Control Ball to Stick Ball Position.\nReset Control Ball's Position
  (set `self.InterpStickRotation` (`SceneComponent.RelativeRotation` (`self.HingePoint`))) ; Set InterpStickRotation from current Rotator
  (bind (_direction `_새_트랙_0`) (`Timeline|타임라인_0` :!via `PlayFromStart`)
    (:`Update`
      (if (not (`self.bIsGrabbed`))
        (`SceneComponent.K2_SetRelativeRotation` (`self.HingePoint`) (`KismetMathLibrary.RLerp` (`self.InterpStickRotation`) (struct) `_새_트랙_0`) false false)
        (`SceneComponent.K2_SetWorldLocationAndRotation` (`self.ControlBall`) (`SceneComponent.K2_GetComponentLocation` _controlpoint) (`SceneComponent.K2_GetComponentRotation` _controlpoint) false false)))))

(event `/Game/VirtualRealityBP/Blueprints/PickupActorInterface.Pickup`
  (params (AttachTo :type "SceneComponent Object Reference"))
  ;[1 1 1] Pickup
  (bind _output_get (set `self.Hand` AttachTo))
  (`SceneComponent.K2_AttachToComponent` (`self.ControlBall`) _output_get "None" "KeepWorld" "KeepWorld" "KeepRelative" false) ; Attach Control Ball to VR Hand
  (set `self.bIsGrabbed` true)
  (`self.Start Tracking`))

(event `self.ReceiveTick`
  (params (DeltaSeconds :type "Float (single-precision)"))
  (set `self.ThrottleValue` (`KismetMathLibrary.MapRangeClamped` (`self.GetTQSAngle`) (`self.AngleMin`) (`self.AngleMax`) 0.0 1.0))
  ;[1 1 1] Tick
  (`/Engine/EditorBlueprintResources/StandardMacros.Gate` true :!label _label
    (:`Exit`
      (set `self.TQSDirection` (`self.GetTQSDirection`)) ; Get the
      (`self.RotateHindge`)
      (if (>= (`self.GetTQSAngle`) (`self.AngleMin`))
        (if (<= (`self.GetTQSAngle`) (`self.AngleMax`))
          (`SceneComponent.K2_SetWorldRotation` (`self.SpinPoint`) (`self.GetTQSRotation`) false false)
          (`SceneComponent.K2_SetRelativeLocation` (`self.SpinPoint`) (`SceneComponent.RelativeLocation` (`self.ResetPoint`)) false false))))))

(event `Start Tracking`
  ;[1 1 1] Tick
  (goto _label :!via `Open`))

(event `Stop Tracking`
  ;[1 1 1] Tick
  (goto _label :!via `Close`))

(fn `GetAnimSequence`
  (params (Hand :type "EControllerHand Enum" :default "Left"))
  (returns (AnimSequence :type "AnimSequence Object Reference"))
  (return null))

(fn `GetLocationStickXAxis`
  (returns (XAxis :type "Vector Structure"))
  (return (`KismetMathLibrary.TransformLocation` (`self.GetTransform`) (`KismetMathLibrary.ProjectVectorOnToVector` (`KismetMathLibrary.InverseTransformLocation` (`self.GetTransform`) (`SceneComponent.K2_GetComponentLocation` (`self.Hand`))) (`KismetMathLibrary.GetForwardVector` (`SceneComponent.RelativeRotation` (`self.FrictionWheel`)))))))

(fn `GetPickupComponent`
  (returns (PickupComponent :type "/Game/Hands/BPC_PickupObject Object Reference"))
  (return null))

(fn `GetTQSAngle`
  (returns (ReturnValue :type "Float (double-precision)"))
  (bind (_returnvalue_x _returnvalue_y) (`KismetMathLibrary.BreakVector` (`KismetMathLibrary.Cross_VectorVector` (`self.InitialUpVector`) (`self.TQSDirection`))))
  (return (* (`KismetMathLibrary.DegAcos` (`KismetMathLibrary.Dot_VectorVector` (`self.InitialUpVector`) (`self.TQSDirection`))) (`KismetMathLibrary.SelectFloat` -1.0 1.0 (< _returnvalue_y 0.0)))))

(fn `GetTQSDirection`
  (returns (ReturnValue :type "Vector Structure"))
  (return (`KismetMathLibrary.Normal` (- (`self.GetLocationStickXAxis`) (`SceneComponent.K2_GetComponentLocation` (`self.SpinPoint`))))))

(fn `GetTQSRotation`
  (returns (NewParam :type "Rotator Structure"))
  (return (`KismetMathLibrary.MakeRotFromZX` (`self.TQSDirection`) (`KismetMathLibrary.RotateAngleAxis` (`self.TQSDirection`) 90.0 (`KismetMathLibrary.GetRightVector` (`SceneComponent.K2_GetComponentRotation` (`self.SpinPoint`)))))))

(fn `GetTQSRotationAtAngle`
  (params (DesireAngle :type "Float (double-precision)"))
  (returns (ReturnValue :type "Rotator Structure"))
  (bind _returnvalue (`KismetMathLibrary.GetRightVector` (`SceneComponent.K2_GetComponentRotation` (`self.Scene`))))
  (bind _returnvalue_2 (`KismetMathLibrary.RotateAngleAxis` (`self.InitialUpVector`) DesireAngle (`KismetMathLibrary.NegateVector` _returnvalue)))
  (return (`KismetMathLibrary.MakeRotFromZX` _returnvalue_2 (`KismetMathLibrary.RotateAngleAxis` _returnvalue_2 90.0 _returnvalue))))

(fn `IsIdleRange`)

(fn `RotateHindge`
  (bind _returnvalue (`KismetMathLibrary.FClamp` (/ (.roll (.rotation (`KismetMathLibrary.ConvertTransformToRelative` (`SceneComponent.K2_GetComponentToWorld` (`self.ControlBall`)) (`SceneComponent.K2_GetComponentToWorld` (`self.ControlPoint`))))) -1.1) 0.0 25.0))
  (`SceneComponent.K2_SetRelativeRotation` (`self.HingePoint`) (`KismetMathLibrary.MakeRotator` _returnvalue) false false)
  (set `self.bIsTurned` (`KismetMathLibrary.NearlyEqual_FloatFloat` _returnvalue 25.0 5.0)))

(fn `SetAfterburner`
  (set `self.bIsIdle` false)
  (set `self.bIsNormal` false)
  (set `self.bIsAfterburner` true)
  (set `self.AngleMin` (`self.AngleAfterMin`))
  (set `self.AngleMax` (`self.AngleAfterMax`)))

(fn `SetIdle`
  (set `self.bIsIdle` true)
  (set `self.bIsNormal` false)
  (set `self.bIsAfterburner` false)
  (set `self.AngleMin` (`self.AngleIdleMin`))
  (set `self.AngleMax` (`self.AngleIdleMax`)))

(fn `SetLimitOfAngleByState`
  (if (`self.bIsIdle`)
    (`self.SetIdle`)
    (elif (`self.bIsNormal`)
      (`self.SetNormal`)
      (elif (`self.bIsAfterburner`)
        (`self.SetAfterburner`)
        (else
          (`KismetSystemLibrary.PrintString` "Hello"))))))

(fn `SetNormal`
  (set `self.bIsIdle` false)
  (set `self.bIsNormal` true)
  (set `self.bIsAfterburner` false)
  (set `self.AngleMin` (`self.AngleIdleMax`))
  (set `self.AngleMax` (`self.AngleAfterMin`)))

(fn `UserConstructionScript`
  (set `self.bIsIdle` true))