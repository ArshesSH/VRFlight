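; VR-grabbable ejection handle for the F-16C that sets an ejection flag when pulled far enough.
; Pickup attaches an invisible control ball to the hand and opens a Tick gate.
; Tick maps the ball's Scene-relative Z to clamped handle travel, setting IsEjectionOn past a threshold.
; Drop snaps the ball back and, unless ejection is on, a timeline lerps the handle from its pickup-time position to zero.
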(event `self.ReceiveBeginPlay`)

(event `/Game/VirtualRealityBP/Blueprints/PickupActorInterface.Pickup`
  (params (AttachTo :type "SceneComponent Object Reference"))
  (bind _controlball (`self.ControlBall`))
  (bind _output_get (set `self.Hand` AttachTo))
  (`SceneComponent.K2_AttachToComponent` _controlball _output_get "None" "KeepWorld" "KeepWorld" "KeepRelative" false) ; Attach Control Ball to VR Hand
  (`SceneComponent.ToggleVisibility` _controlball false)
  (set `self.bIsGrabbed` true)
  (set `self.InterpStickLocation` (`SceneComponent.RelativeLocation` (`self.ControlPoint`)))
  (`self.Start Tracking`))

(event `/Game/VirtualRealityBP/Blueprints/PickupActorInterface.Drop`
  (bind _controlball (`self.ControlBall`))
  (bind _controlballposition (`self.ControlBallPosition`))
  (`self.Stop Tracking`)
  (set `self.Hand` null)
  (set `self.bIsGrabbed` false)
  (`SceneComponent.ToggleVisibility` _controlball false)
  (`SceneComponent.K2_DetachFromComponent` _controlball "KeepWorld" "KeepWorld" "KeepWorld" false) ; Detach Control Ball from VR Hand
  (`SceneComponent.K2_AttachToComponent` _controlball (`self.ControlBallPosition`) "None" "KeepRelative" "KeepRelative" "KeepRelative" false) ; Attach Control Ball to Stick Ball Position.\nReset Control Ball's Position
  (`SceneComponent.K2_SetWorldLocationAndRotation` (`self.ControlBall`) (`SceneComponent.K2_GetComponentLocation` _controlballposition) (`SceneComponent.K2_GetComponentRotation` _controlballposition) false false)
  (if (not (`self.bIsEjectionOn`))
    (bind (_direction `_새_트랙_0`) (`Timeline|타임라인_0` :!via `PlayFromStart`) ; Start reset Stick Position
      (:`Update`
        (if (not (`self.bIsGrabbed`))
          (`SceneComponent.K2_SetRelativeLocation` (`self.ControlPoint`) (`KismetMathLibrary.VLerp` (`self.InterpStickLocation`) (0.0 0.0 0.0) `_새_트랙_0`) false false))))))

(event `self.ReceiveTick`
  (params (DeltaSeconds :type "Float (single-precision)"))
  (bind (_relativerotation_roll _relativerotation_pitch) (`KismetMathLibrary.BreakRotator` (`SceneComponent.RelativeRotation` (`self.ControlPoint`))))
  (bind _returnvalue (`KismetMathLibrary.FClamp` (/ (.z (.location (`KismetMathLibrary.ConvertTransformToRelative` (`SceneComponent.K2_GetComponentToWorld` (`self.ControlBall`)) (`SceneComponent.K2_GetComponentToWorld` (`self.Scene`))))) -7.0) 0.0 30.0))
  (`/Engine/EditorBlueprintResources/StandardMacros.Gate` true :!label _label
    (:`Exit`
      (`SceneComponent.K2_SetRelativeLocation` (`self.ControlPoint`) (`KismetMathLibrary.MakeVector` _relativerotation_roll _relativerotation_pitch _returnvalue) false false)
      (if (> _returnvalue 20.0)
        (set `self.bIsEjectionOn` true)
        (else
          (set `self.bIsEjectionOn` false))))))

(event `Start Tracking`
  (goto _label :!via `Open`))

(event `Stop Tracking`
  (goto _label :!via `Close`))

(fn `GetAnimSequence`
  (params (Hand :type "EControllerHand Enum" :default "Left"))
  (returns (AnimSequence :type "AnimSequence Object Reference"))
  (return null))

(fn `GetLocationStickXAxis`
  (returns (XAxis :type "Vector Structure"))
  (return (0.0 0.0 0.0)))

(fn `GetPickupComponent`
  (returns (PickupComponent :type "/Game/Hands/BPC_PickupObject Object Reference"))
  (return null))

(fn `GetStickDirection`
  (returns (ReturnValue :type "Vector Structure"))
  (return (`KismetMathLibrary.Normal` (- (`self.GetLocationStickXAxis`) (`SceneComponent.K2_GetComponentLocation` (`self.ControlPoint`))))))

(fn `UserConstructionScript`)