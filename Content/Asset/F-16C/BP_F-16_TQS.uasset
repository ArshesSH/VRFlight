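; VR-grabbable F-16 throttle (TQS) with idle, normal and afterburner angle ranges, apparently unfinished.
; Pickup attaches a control ball to the hand; drop reattaches it and a timeline eases the hinge rotation back.
; RotateStick converts ball offset and roll into clamped spin, hinge twist and throttle value, but is never run.
; While held, gated Tick only updates state flags; the switch to the normal range is disabled by a false condition.
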(event `/Game/VirtualRealityBP/Blueprints/PickupActorInterface.Pickup`
  (params (AttachTo :type "SceneComponent Object Reference"))
  (bind _controlball (`self.ControlBall`))
  ;[1 1 1] Pickup
  (`SceneComponent.K2_AttachToComponent` _controlball AttachTo "None" "KeepWorld" "KeepWorld" "KeepRelative" false) ; Attach Control Ball to VR Hand
  (`SceneComponent.ToggleVisibility` _controlball false)
  (set `self.bIsGrabbed` true)
  (`self.Start Tracking`))

(event `/Game/VirtualRealityBP/Blueprints/PickupActorInterface.Drop`
  (bind _controlpoint (`self.ControlPoint`))
  (bind _controlball (`self.ControlBall`))
  ;[1 1 1] Drop
  (`self.Stop Tracking`)
  (set `self.bIsGrabbed` false)
  (`SceneComponent.ToggleVisibility` _controlball false)
  (`SceneComponent.K2_DetachFromComponent` _controlball "KeepWorld" "KeepWorld" "KeepWorld" false) ; Detach Control Ball from VR Hand
  (`SceneComponent.K2_AttachToComponent` _controlball null "None" "KeepRelative" "KeepRelative" "KeepRelative" false) ; Attach Control Ball to Stick Ball Position.\nReset Control Ball's Position
  (set `self.InterpStickRotation` (`SceneComponent.RelativeRotation` (`self.HingePoint`))) ; Set InterpStickRotation from current Rotator
  (bind (_direction `_새_트랙_0`) (`Timeline|Reset` :!via `PlayFromStart`)
    (:`Update`
      (if (not (`self.bIsGrabbed`))
        (`SceneComponent.K2_SetRelativeRotation` (`self.HingePoint`) (`KismetMathLibrary.RLerp` (`self.InterpStickRotation`) (struct) `_새_트랙_0`) false false)
        (`SceneComponent.K2_SetWorldLocationAndRotation` (`self.ControlBall`) (`SceneComponent.K2_GetComponentLocation` _controlpoint) (`SceneComponent.K2_GetComponentRotation` _controlpoint) false false)))))

(event `self.ReceiveTick`
  (params (DeltaSeconds :type "Float (single-precision)"))
  (bind (_relativerotation_roll _relativerotation_pitch) (`KismetMathLibrary.BreakRotator` (`SceneComponent.RelativeRotation` (`self.SpinPoint`))))
  (`/Engine/EditorBlueprintResources/StandardMacros.Gate` true :!label _label
    (:`Exit`
      (`|ExecutionSequence`
        (:`then_0`
          (`self.DetectState`))
        (:`then_1`
          (if (and (`KismetMathLibrary.NearlyEqual_FloatFloat` _relativerotation_pitch (`self.AngleIdleMax`) 1.0) (and (`self.bIsIdle`) false))
            (`self.SetNormal`)))))))

(event `Start Tracking`
  (goto _label :!via `Open`))

(event `Stop Tracking`
  (goto _label :!via `Close`))

(fn `DetectState`
  (bind (_relativerotation_roll _relativerotation_pitch) (`KismetMathLibrary.BreakRotator` (`SceneComponent.RelativeRotation` (`self.SpinPoint`))))
  (bind _output_get (set `self.bIsIdle` (`KismetMathLibrary.InRange_FloatFloat` _relativerotation_pitch (`self.AngleIdleMin`) (`self.AngleIdleMax`))))
  (set `self.bIsNormal` (`KismetMathLibrary.InRange_FloatFloat` _relativerotation_pitch (`self.AngleIdleMin`) (`self.AngleAfterMax`) false false))
  (set `self.bIsAfterburner` _output_get))

(fn `GetAnimSequence`
  (params (Hand :type "EControllerHand Enum" :default "Left"))
  (returns (AnimSequence :type "AnimSequence Object Reference"))
  (return null))

(fn `GetPickupComponent`
  (returns (PickupComponent :type "/Game/Hands/BPC_PickupObject Object Reference"))
  (return null))

(fn `IsIdleRange`)

(fn `RotateStick`
  (bind _returnvalue (`KismetMathLibrary.ConvertTransformToRelative` (`SceneComponent.K2_GetComponentToWorld` (`self.ControlBall`)) (`SceneComponent.K2_GetComponentToWorld` (`self.ControlPoint`))))
  (bind _returnvalue_2 (`KismetMathLibrary.FClamp` (/ (.x (.location _returnvalue)) 5.0) (`self.AngleMin`) (`self.AngleMax`)))
  (bind _returnvalue_3 (`KismetMathLibrary.FClamp` (/ (.roll (.rotation _returnvalue)) -3.0) 0.0 25.0))
  (`SceneComponent.K2_SetRelativeRotation` (`self.SpinPoint`) (`KismetMathLibrary.MakeRotator` 0.0 _returnvalue_2) false false)
  (`SceneComponent.K2_SetRelativeRotation` (`self.HingePoint`) (`KismetMathLibrary.MakeRotator` _returnvalue_3) false false)
  (set `self.ThrottleValue` (`KismetMathLibrary.MapRangeClamped` _returnvalue_2 -35.0 35.0 0.0 1.0))
  (set `self.bIsTurned` (`KismetMathLibrary.NearlyEqual_FloatFloat` _returnvalue_3 25.0 5.0)))

(fn `SetAfterburner`
  (set `self.bIsIdle` false)
  (set `self.bIsNormal` false)
  (set `self.bIsAfterburner` true)
  (set `self.AngleMin` (`self.AngleAfterMin`))
  (set `self.AngleMax` (`self.AngleAfterMax`)))

(fn `SetIdle`
  (set `self.bIsIdle` true)
  (set `self.bIsNormal` false)
  (set `self.bIsAfterburner` false)
  (set `self.AngleMin` (`self.AngleIdleMin`))
  (set `self.AngleMax` (`self.AngleIdleMax`)))

(fn `SetNormal`
  (set `self.AngleMin` (`self.AngleIdleMax`))
  (set `self.AngleMax` (`self.AngleAfterMin`)))

(fn `UserConstructionScript`
  (set `self.bIsIdle` true)
  (`SceneComponent.K2_SetRelativeRotation` (`self.SpinPoint`) (`KismetMathLibrary.MakeRotator` 0.0 (`self.AngleIdleMin`)) false false))