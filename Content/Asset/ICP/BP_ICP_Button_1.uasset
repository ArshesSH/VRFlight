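; ICP button 1 actor, a cockpit panel key that switches pages on the DED display.
; ButtonAction reads the page flags on DEDWidget, turning the main page into TILS and the List page into DEST1.
; Each switch toggles the visibility of the two page components and updates their flags, so the key's function depends on the current page.
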(event `self.ButtonAction`
  (`|ExecutionSequence`
    (:`then_0`
      (if (`/Game/ded/BP_DED.bIsDED_Main` (`self.DED_Widget`))
        (`SceneComponent.SetVisibility` (`/Game/ded/BP_DED.DED_Main` (`self.DED_Widget`)) false false)
        (`SceneComponent.SetVisibility` (`/Game/ded/BP_DED.DED_TILS` (`self.DED_Widget`)) true false)
        (set `/Game/ded/BP_DED.bIsDED_Main` false (`self.DED_Widget`))
        (set `/Game/ded/BP_DED.bIsDED_TILS` true (`self.DED_Widget`))))
    (:`then_1`
      (if (`/Game/ded/BP_DED.bIsDED_List` (`self.DED_Widget`))
        (`SceneComponent.SetVisibility` (`/Game/ded/BP_DED.DED_List` (`self.DED_Widget`)) false false)
        (`SceneComponent.SetVisibility` (`/Game/ded/BP_DED.DED_Dest1` (`self.DED_Widget`)) true false)
        (set `/Game/ded/BP_DED.bIsDED_List` false (`self.DED_Widget`))
        (set `/Game/ded/BP_DED.bIsDED_DEST_1` true (`self.DED_Widget`))))))

(fn `UserConstructionScript`
  (`parent.UserConstructionScript`))