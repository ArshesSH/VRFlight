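; BP_ICP_Button_Enter is the Enter button on the F-16C's ICP, which toggles ILS mode.
; On BeginPlay it runs the parent logic and caches the player pawn as the F-16C.
; ButtonAction acts only while the DED widget's IsDEDTILS flag is set.
; It then flips the aircraft's ILSOn state, setting HUD ILS visibility and the HSI frequency-match flag to the same value.
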(event `self.ReceiveBeginPlay`
  (`parent.ReceiveBeginPlay`)
  (bind _asbp_f_16c (cast `/Game/Asset/F-16C/BP_F-16C` (`GameplayStatics.GetPlayerPawn` 0)))
  (set `self.As BP F-16C` _asbp_f_16c))

(event `self.ButtonAction`
  (bind _as_bp_f_16c (`self.As BP F-16C`))
  (bind _as_bp_f_16c_2 (`self.As BP F-16C`))
  (if (`/Game/ded/BP_DED.bIsDED_TILS` (`self.DED_Widget`))
    (if (`/Game/Asset/F-16C/BP_F-16C.bILSOn` (`self.As BP F-16C`))
      (set `/Game/Asset/F-16C/BP_F-16C.bILSOn` false _as_bp_f_16c)
      (`SceneComponent.SetVisibility` (`/Game/Asset/F-16C/BP_F-16C.HUD_ILS` _as_bp_f_16c) false false)
      (set `/Game/Flight_Instrument_Pack/Widgets/InstrumentWidgets/HSI_Widget/HSI_Blueprint_3.Is_Match_Freq` false (`/Game/Asset/F-16C/BP_F-16C.HSI_Var` (`self.As BP F-16C`)))
      (else
        (set `/Game/Asset/F-16C/BP_F-16C.bILSOn` true _as_bp_f_16c_2)
        (`SceneComponent.SetVisibility` (`/Game/Asset/F-16C/BP_F-16C.HUD_ILS` _as_bp_f_16c_2) true false)
        (set `/Game/Flight_Instrument_Pack/Widgets/InstrumentWidgets/HSI_Widget/HSI_Blueprint_3.Is_Match_Freq` true (`/Game/Asset/F-16C/BP_F-16C.HSI_Var` (`self.As BP F-16C`)))))))

(fn `UserConstructionScript`
  (`parent.UserConstructionScript`))