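; HUD instrument landing system indicator that shows the player aircraft's deviation through localizer and glideslope markers.
; On BeginPlay it caches a BP_ILS actor from the level, keeping the last one found.
; Each tick it rotates that ILS Position component to the player-to-ILS look-at rotation.
; Yaw and pitch differences against the player's rotation, clamped and remapped, slide LocalizerPoint and GlideSlopePoint.
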(event `self.ReceiveBeginPlay`
  (bind _outactors (`GameplayStatics.GetAllActorsOfClass` "/Game/Flight_Instrument_Pack/Widgets/InstrumentWidgets/HSI_Widget/BP_ILS.BP_ILS_C"))
  (for _array_element _outactors
    (set `self.ILS_Instruement` _array_element)))

(event `self.ReceiveTick`
  (params (DeltaSeconds :type "Float (single-precision)"))
  (bind (_returnvalue_roll _returnvalue_pitch _returnvalue_yaw) (`KismetMathLibrary.BreakRotator` (`SceneComponent.K2_GetComponentRotation` (`Actor.RootComponent` (`GameplayStatics.GetPlayerPawn` 0)))))
  (bind (_returnvalue_roll_2 _returnvalue_pitch_2 _returnvalue_yaw_2) (`KismetMathLibrary.BreakRotator` (`SceneComponent.K2_GetComponentRotation` (`/Game/Flight_Instrument_Pack/Widgets/InstrumentWidgets/HSI_Widget/BP_ILS.Position` (`self.ILS_Instruement`)))))
  (`SceneComponent.K2_SetRelativeRotation` (`/Game/Flight_Instrument_Pack/Widgets/InstrumentWidgets/HSI_Widget/BP_ILS.Position` (`self.ILS_Instruement`)) (`KismetMathLibrary.FindLookAtRotation` (`SceneComponent.K2_GetComponentLocation` (`Actor.RootComponent` (`GameplayStatics.GetPlayerPawn` 0))) (`SceneComponent.K2_GetComponentLocation` (`/Game/Flight_Instrument_Pack/Widgets/InstrumentWidgets/HSI_Widget/BP_ILS.Position` (`self.ILS_Instruement`)))) false false)
  (`SceneComponent.K2_SetRelativeLocation` (`self.LocalizerPoint`) (`KismetMathLibrary.MakeVector` 0.0 (`KismetMathLibrary.MapRangeClamped` (- _returnvalue_yaw _returnvalue_yaw_2) -22.0 22.0 -100.0 100.0)) false false)
  (`SceneComponent.K2_SetRelativeLocation` (`self.GlideSlopePoint`) (`KismetMathLibrary.MakeVector` (`KismetMathLibrary.MapRangeClamped` (- _returnvalue_pitch_2 _returnvalue_pitch) 0.0 6.0 -10.0 10.0)) false false))

(fn `UserConstructionScript`)