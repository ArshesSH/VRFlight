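; BP_ICP_Button_LIST is the LIST button on a cockpit ICP, which switches the DED display to its List page.
; Its ButtonAction event shows the List element on DEDWidget and hides the Main, OA1, TILS and five Dest pages.
; It then sets the widget's matching page-state booleans so only IsDEDList is true, hard-coding every page rather than using a shared page switcher.
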(event `self.ButtonAction`
  (`SceneComponent.SetVisibility` (`/Game/ded/BP_DED.DED_Main` (`self.DED_Widget`)) false false)
  (`SceneComponent.SetVisibility` (`/Game/ded/BP_DED.DED_List` (`self.DED_Widget`)) true false)
  (`SceneComponent.SetVisibility` (`/Game/ded/BP_DED.DED_OA1` (`self.DED_Widget`)) false false)
  (`SceneComponent.SetVisibility` (`/Game/ded/BP_DED.DED_TILS` (`self.DED_Widget`)) false false)
  (`SceneComponent.SetVisibility` (`/Game/ded/BP_DED.DED_Dest1` (`self.DED_Widget`)) false false)
  (`SceneComponent.SetVisibility` (`/Game/ded/BP_DED.DED_Dest2` (`self.DED_Widget`)) false false)
  (`SceneComponent.SetVisibility` (`/Game/ded/BP_DED.DED_Dest3` (`self.DED_Widget`)) false false)
  (`SceneComponent.SetVisibility` (`/Game/ded/BP_DED.DED_Dest4` (`self.DED_Widget`)) false false)
  (`SceneComponent.SetVisibility` (`/Game/ded/BP_DED.DED_Dest5` (`self.DED_Widget`)) false false)
  (set `/Game/ded/BP_DED.bIsDED_Main` false (`self.DED_Widget`))
  (set `/Game/ded/BP_DED.bIsDED_List` true (`self.DED_Widget`))
  (set `/Game/ded/BP_DED.bIsDED_OA1` false (`self.DED_Widget`))
  (set `/Game/ded/BP_DED.bIsDED_TILS` false (`self.DED_Widget`))
  (set `/Game/ded/BP_DED.bIsDED_DEST_1` false (`self.DED_Widget`))
  (set `/Game/ded/BP_DED.bIsDED_DEST_2` false (`self.DED_Widget`))
  (set `/Game/ded/BP_DED.bIsDED_DEST_3` false (`self.DED_Widget`))
  (set `/Game/ded/BP_DED.bIsDED_DEST_4` false (`self.DED_Widget`))
  (set `/Game/ded/BP_DED.bIsDED_DEST_5` false (`self.DED_Widget`)))

(fn `UserConstructionScript`
  (`parent.UserConstructionScript`))