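; VR-grabbable four-way ICP switch in the F-16C cockpit that changes pages on the DED display.
; While held, a gated Tick converts the hand-attached ControlBall's relative position into clamped SpinPoint tilt, snapping near the limits and latching a direction.
; On release, a timeline springs the switch back and applies that direction: left shows the main page, right opens OA1 from main, up/down cycle the five DEST pages.
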(event `self.ReceiveBeginPlay`
  (bind _asbp_f_16c (cast `/Game/untitled_category/untitled_asset/F-16C/BP_F-16C` (`GameplayStatics.GetPlayerPawn` 0)))
  (bind _asbp_ded (cast `/Game/ded/BP_DED` (`ChildActorComponent.ChildActor` (`/Game/untitled_category/untitled_asset/F-16C/BP_F-16C.DED` _asbp_f_16c))))
  (set `self.DED_Widget` _asbp_ded))

(event `/Game/VirtualRealityBP/Blueprints/PickupActorInterface.Pickup`
  (params (AttachTo :type "SceneComponent Object Reference"))
  (bind _output_get (set `self.Hand` AttachTo))
  (`SceneComponent.ToggleVisibility` (`self.ControlBall`) false)
  (set `self.bIsGrabbed` true)
  (`SceneComponent.K2_AttachToComponent` (`self.ControlBall`) _output_get "None" "KeepWorld" "KeepWorld" "KeepRelative" false) ; Attach Control Ball to VR Hand
  (`self.StartTick`))

(event `/Game/VirtualRealityBP/Blueprints/PickupActorInterface.Drop`
  (bind _controlballpositon (`self.ControlBallPositon`))
  (`self.StopTick`)
  (set `self.Hand` null)
  (set `self.bIsGrabbed` false)
  (set `self.InterpRotator` (`SceneComponent.RelativeRotation` (`self.SpinPoint`)))
  (`SceneComponent.ToggleVisibility` (`self.ControlBall`) false)
  (`SceneComponent.K2_DetachFromComponent` (`self.ControlBall`) "KeepWorld" "KeepWorld" "KeepWorld" false) ; Detach Control Ball from VR Hand
  (`SceneComponent.K2_AttachToComponent` (`self.ControlBall`) (`self.ControlBallPositon`) "None" "KeepRelative" "KeepRelative" "KeepRelative" false) ; Attach Control Ball to Stick Ball Position.\nReset Control Ball's Position
  (`SceneComponent.K2_SetWorldLocationAndRotation` (`self.ControlBall`) (`SceneComponent.K2_GetComponentLocation` _controlballpositon) (`SceneComponent.K2_GetComponentRotation` _controlballpositon) false false)
  (bind (_direction `_새_트랙_0`) (`Timeline|타임라인_0` :!via `PlayFromStart`)
    (:`Update`
      (if (not (`self.bIsGrabbed`))
        (`SceneComponent.K2_SetRelativeRotation` (`self.SpinPoint`) (`KismetMathLibrary.RLerp` (`self.InterpRotator`) (struct) `_새_트랙_0`) false false)
        (`|ExecutionSequence`
          (:`then_0`
            (if (`self.bInputLeft`)
              (`SceneComponent.SetVisibility` (`/Game/ded/BP_DED.DED_Main` (`self.DED_Widget`)) true false)
              (`SceneComponent.SetVisibility` (`/Game/ded/BP_DED.DED_List` (`self.DED_Widget`)) false false)
              (`SceneComponent.SetVisibility` (`/Game/ded/BP_DED.DED_OA1` (`self.DED_Widget`)) false false)
              (`SceneComponent.SetVisibility` (`/Game/ded/BP_DED.DED_TILS` (`self.DED_Widget`)) false false)
              (`SceneComponent.SetVisibility` (`/Game/ded/BP_DED.DED_Dest1` (`self.DED_Widget`)) false false)
              (`SceneComponent.SetVisibility` (`/Game/ded/BP_DED.DED_Dest2` (`self.DED_Widget`)) false false)
              (`SceneComponent.SetVisibility` (`/Game/ded/BP_DED.DED_Dest3` (`self.DED_Widget`)) false false)
              (`SceneComponent.SetVisibility` (`/Game/ded/BP_DED.DED_Dest4` (`self.DED_Widget`)) false false)
              (`SceneComponent.SetVisibility` (`/Game/ded/BP_DED.DED_Dest5` (`self.DED_Widget`)) false false)
              (set `/Game/ded/BP_DED.bIsDED_Main` true (`self.DED_Widget`))
              (set `/Game/ded/BP_DED.bIsDED_List` false (`self.DED_Widget`))
              (set `/Game/ded/BP_DED.bIsDED_OA1` false (`self.DED_Widget`))
              (set `/Game/ded/BP_DED.bIsDED_TILS` false (`self.DED_Widget`))
              (set `/Game/ded/BP_DED.bIsDED_DEST_1` false (`self.DED_Widget`))
              (set `/Game/ded/BP_DED.bIsDED_DEST_2` false (`self.DED_Widget`))
              (set `/Game/ded/BP_DED.bIsDED_DEST_3` false (`self.DED_Widget`))
              (set `/Game/ded/BP_DED.bIsDED_DEST_4` false (`self.DED_Widget`))
              (set `/Game/ded/BP_DED.bIsDED_DEST_5` false (`self.DED_Widget`))
              (set `self.bInputLeft` true)))
          (:`then_1`
            (if (`/Game/ded/BP_DED.bIsDED_Main` (`self.DED_Widget`))
              (if (`self.bInputRight`)
                (`SceneComponent.SetVisibility` (`/Game/ded/BP_DED.DED_Main` (`self.DED_Widget`)) false false)
                (`SceneComponent.SetVisibility` (`/Game/ded/BP_DED.DED_OA1` (`self.DED_Widget`)) true false)
                (set `/Game/ded/BP_DED.bIsDED_Main` false (`self.DED_Widget`))
                (set `/Game/ded/BP_DED.bIsDED_OA1` true (`self.DED_Widget`))
                (set `self.bInputRight` false))))
          (:`then_2`
            (if (`self.bInputUp`)
              (`self.DED_Up`)))
          (:`then_3`
            (if (`self.bInputDown`)
              (`self.DED_Down`))))))))

(event `self.ReceiveTick`
  (params (DeltaSeconds :type "Float (single-precision)"))
  (bind _returnvalue (`KismetMathLibrary.ConvertTransformToRelative` (`SceneComponent.K2_GetComponentToWorld` (`self.ControlBall`)) (`SceneComponent.K2_GetComponentToWorld` (`self.Scene`))))
  (bind _returnvalue_2 (`KismetMathLibrary.FClamp` (/ (.y (.location _returnvalue)) -5.0) -25.0 25.0))
  (bind _returnvalue_3 (`KismetMathLibrary.FClamp` (/ (.x (.location _returnvalue)) 5.0) -25.0 25.0))
  (`/Engine/EditorBlueprintResources/StandardMacros.Gate` true :!label _label
    (:`Exit`
      (set `self.YAxis` _returnvalue_3)
      (set `self.XAxis` _returnvalue_2)
      (`SceneComponent.K2_SetRelativeRotation` (`self.SpinPoint`) (`KismetMathLibrary.MakeRotator` 0.0 _returnvalue_3 _returnvalue_2) false false)
      (`|ExecutionSequence`
        (:`then_1`
          (if (`KismetMathLibrary.InRange_FloatFloat` (`self.XAxis`) 15.0 25.0)
            (`SceneComponent.K2_SetRelativeRotation` (`self.SpinPoint`) (`KismetMathLibrary.MakeRotator` 0.0 0.0 25.0) false false)
            (set `self.bInputRight` false)
            (set `self.bInputLeft` true)
            (set `self.bInputUp` false)
            (set `self.bInputDown` false)))
        (:`then_2`
          (if (`KismetMathLibrary.InRange_FloatFloat` (`self.XAxis`) -25.0 -15.0)
            (`SceneComponent.K2_SetRelativeRotation` (`self.SpinPoint`) (`KismetMathLibrary.MakeRotator` 0.0 0.0 -25.0) false false)
            (set `self.bInputRight` true)
            (set `self.bInputLeft` false)
            (set `self.bInputUp` false)
            (set `self.bInputDown` false)))
        (:`then_3`
          (if (`KismetMathLibrary.InRange_FloatFloat` (`self.YAxis`) -25.0 -15.0)
            (`SceneComponent.K2_SetRelativeRotation` (`self.SpinPoint`) (`KismetMathLibrary.MakeRotator` 0.0 -25.0) false false)
            (set `self.bInputRight` false)
            (set `self.bInputLeft` false)
            (set `self.bInputUp` false)
            (set `self.bInputDown` true)))
        (:`then_4`
          (if (`KismetMathLibrary.InRange_FloatFloat` (`self.YAxis`) 15.0 25.0)
            (`SceneComponent.K2_SetRelativeRotation` (`self.SpinPoint`) (`KismetMathLibrary.MakeRotator` 0.0 25.0) false false)
            (set `self.bInputRight` false)
            (set `self.bInputLeft` false)
            (set `self.bInputUp` true)
            (set `self.bInputDown` false)))))))

(event `StartTick`
  (goto _label :!via `Open`))

(event `StopTick`
  (goto _label :!via `Close`))

(fn `GetAnimSequence`
  (params (Hand :type "EControllerHand Enum" :default "Left"))
  (returns (AnimSequence :type "AnimSequence Object Reference"))
  (return null))

(fn `GetPickupComponent`
  (returns (PickupComponent :type "/Game/Hands/BPC_PickupObject Object Reference"))
  (return null))

(fn `UserConstructionScript`)