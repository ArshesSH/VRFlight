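; VR-grabbable F-16 flight stick that tilts with the player's hand and springs back to neutral on release.
; Pickup attaches a proxy ControlBall to the hand; while grabbed, Tick turns its inverted rotation, relative to Scene, into clamped StickPoint rotation and saves it as StickRotator.
; Drop reattaches the ball to StickBallPosition, and the Reset timeline lerps the stick back to zero rotation.
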(event `/Game/VirtualRealityBP/Blueprints/PickupActorInterface.Pickup`
  (params (AttachTo :type "SceneComponent Object Reference"))
  (bind _controlball (`self.ControlBall`))
  ;[1 1 1] Pick Up
  (set `self.IsGrabbed` true) ; Set IsGrabbed to True
  (`SceneComponent.K2_AttachToComponent` _controlball AttachTo "None" "KeepWorld" "KeepWorld" "KeepRelative" false) ; Attach Control Ball to VR Hand
  (`SceneComponent.ToggleVisibility` _controlball false)
  (`self.StartPickup`))

(event `/Game/VirtualRealityBP/Blueprints/PickupActorInterface.Drop`
  (bind _controlball (`self.ControlBall`))
  (bind _stickballposition (`self.StickBallPosition`))
  ;[1 1 1] Drop
  (set `self.IsGrabbed` false) ; Set IsGrabbed False
  (`SceneComponent.ToggleVisibility` _controlball false)
  (`SceneComponent.K2_DetachFromComponent` _controlball "KeepWorld" "KeepWorld" "KeepWorld" false) ; Detach Control Ball from VR Hand
  (`SceneComponent.K2_AttachToComponent` _controlball (`self.StickBallPosition`) "None" "KeepRelative" "KeepRelative" "KeepRelative" false) ; Attach Control Ball to Stick Ball Position.\nReset Control Ball's Position
  (set `self.ResetRotation` true) ; Set ResetRotation True
  (set `self.InterpStickRotation` (`SceneComponent.RelativeRotation` (`self.StickPoint`))) ; Set InterpStickRotation from current Rotator
  (bind (_direction `_새_트랙_0`) (`Timeline|Reset` :!via `PlayFromStart`) ; Start reset Stick Position
    (:`Update`
      (if (`self.IsGrabbed`)
        (set `self.ResetRotation` false)
        (else
          (`SceneComponent.K2_SetRelativeRotation` (`self.StickPoint`) (`KismetMathLibrary.RLerp` (`self.InterpStickRotation`) (struct) `_새_트랙_0`) false false)
          (`SceneComponent.K2_SetWorldLocationAndRotation` (`self.ControlBall`) (`SceneComponent.K2_GetComponentLocation` _stickballposition) (`SceneComponent.K2_GetComponentRotation` _stickballposition) false false))))
    (:`Finished`
      (`self.StartDrop`))))

(event `self.ReceiveTick`
  (params (DeltaSeconds :type "Float (single-precision)"))
  (bind _stickpoint (`self.StickPoint`))
  (bind _returnvalue (`KismetMathLibrary.ConvertTransformToRelative` (`SceneComponent.K2_GetComponentToWorld` (`self.ControlBall`)) (`SceneComponent.K2_GetComponentToWorld` (`self.Scene`))))
  ;[1 1 1] Grab
  (if (`self.IsGrabbed`) :!label _label
    (`SceneComponent.K2_SetRelativeRotation` _stickpoint (`KismetMathLibrary.MakeRotator` (`KismetMathLibrary.FClamp` (- 0.0 (.roll (.rotation _returnvalue))) -25.0 25.0) (`KismetMathLibrary.FClamp` (- 0.0 (.pitch (.rotation _returnvalue))) -25.0 25.0) (`KismetMathLibrary.FClamp` (- 0.0 (.yaw (.rotation _returnvalue))) -25.0 25.0)) false false)
    (set `self.StickRotator` (`SceneComponent.RelativeRotation` _stickpoint))))

(event `StartPickup`
  ;[1 1 1] Grab
  (`/Engine/EditorBlueprintResources/StandardMacros.Gate` true :!via `Open` :!label _label_2
    (:`Exit`
      (goto _label))))

(event `StartDrop`
  ;[1 1 1] Grab
  (goto _label_2 :!via `Close`))

(fn `GetAnimSequence`
  (params (Hand :type "EControllerHand Enum" :default "Left"))
  (returns (AnimSequence :type "AnimSequence Object Reference"))
  (return null))

(fn `GetPickupComponent`
  (returns (PickupComponent :type "/Game/Hands/BPC_PickupObject Object Reference"))
  (return null))

(fn `UserConstructionScript`)