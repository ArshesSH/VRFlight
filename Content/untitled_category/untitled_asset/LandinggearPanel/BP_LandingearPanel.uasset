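; Cockpit landing gear panel for the F-16C, with a grabbable parking brake switch and three gear indicator lights.
; Pickup shows the control ball and caches switch rotation; Drop hides it, flips the state and eases the switch over with a timeline lerp.
; Each flip turns the parking brake on or off on the player's F-16C pawn, cached at BeginPlay.
; The construction script poses the switch from its initial state; LightOn/LightOff swap light materials.
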(event `self.ReceiveBeginPlay`
  (bind _asbp_f_16c (cast `/Game/untitled_category/untitled_asset/F-16C/BP_F-16C` (`GameplayStatics.GetPlayerPawn` 0)))
  (set `self.As BP F-16C` _asbp_f_16c))

(event `/Game/VirtualRealityBP/Blueprints/PickupActorInterface.Pickup`
  (params (AttachTo :type "SceneComponent Object Reference"))
  (`SceneComponent.SetVisibility` (`self.ParkingBrakeControlBall`) true false)
  (set `self.InterpPBSwitchRotation` (`SceneComponent.RelativeRotation` (`self.ParkingBrakeTogglePoint`))))

(event `/Game/VirtualRealityBP/Blueprints/PickupActorInterface.Drop`
  (`SceneComponent.SetVisibility` (`self.ParkingBrakeControlBall`) false false)
  (if (`self.ParkingBrakeIsUp`)
    (set `self.ParkingBrakeDefaultPos` 15.0)
    (set `self.ParkingBrakeIsUp` false)
    (`self.SwitchDown`)
    (bind (_direction `_새_트랙_0`) (`Timeline|타임라인_0` :!via `PlayFromStart` :!label _label)
      (:`Update`
        (`SceneComponent.K2_SetRelativeRotation` (`self.ParkingBrakeTogglePoint`) (`KismetMathLibrary.RLerp` (`self.InterpPBSwitchRotation`) (`KismetMathLibrary.MakeRotator` (`self.ParkingBrakeDefaultPos`)) `_새_트랙_0`) false false)))
    (else
      (set `self.ParkingBrakeDefaultPos` 0.0)
      (set `self.ParkingBrakeIsUp` true)
      (`self.SwitchUp`)
      (goto _label :!via `PlayFromStart`))))

(event `SwitchUp`
  (`/Game/untitled_category/untitled_asset/F-16C/BP_F-16C.Parking Brake On` (`self.As BP F-16C`)))

(event `SwitchDown`
  (`/Game/untitled_category/untitled_asset/F-16C/BP_F-16C.Parking Brake Off` (`self.As BP F-16C`)))

(fn `GetAnimSequence`
  (params (Hand :type "EControllerHand Enum" :default "Left"))
  (returns (AnimSequence :type "AnimSequence Object Reference"))
  (return null))

(fn `GetPickupComponent`
  (returns (PickupComponent :type "/Game/Hands/BPC_PickupObject Object Reference"))
  (return null))

(fn `LightOff`
  (`PrimitiveComponent.SetMaterial` (`self.LandingGearLight1`) 0 "/Game/AeroComp/Showcase/Meshes/Aircraft/Ju87/black_material.black_material")
  (`PrimitiveComponent.SetMaterial` (`self.LandingGearLight2`) 0 "/Game/AeroComp/Showcase/Meshes/Aircraft/Ju87/black_material.black_material")
  (`PrimitiveComponent.SetMaterial` (`self.LandingGearLight3`) 0 "/Game/AeroComp/Showcase/Meshes/Aircraft/Ju87/black_material.black_material"))

(fn `LightOn`
  (`PrimitiveComponent.SetMaterial` (`self.LandingGearLight1`) 0 "/Game/untitled_category/untitled_asset/LandinggearPanel/GreenLight.GreenLight")
  (`PrimitiveComponent.SetMaterial` (`self.LandingGearLight2`) 0 "/Game/untitled_category/untitled_asset/LandinggearPanel/GreenLight.GreenLight")
  (`PrimitiveComponent.SetMaterial` (`self.LandingGearLight3`) 0 "/Game/untitled_category/untitled_asset/LandinggearPanel/GreenLight.GreenLight"))

(fn `UserConstructionScript`
  (if (`self.ParkingBrakeIsUp`)
    (`SceneComponent.K2_SetRelativeRotation` :`self` (`self.ParkingBrakeTogglePoint`))
    (set `self.ParkingBrakeDefaultPos` 0.0)
    (else
      (`SceneComponent.K2_SetRelativeRotation` (`self.ParkingBrakeTogglePoint`) (struct :`Roll` 15.0) false false)
      (set `self.ParkingBrakeDefaultPos` 15.0))))