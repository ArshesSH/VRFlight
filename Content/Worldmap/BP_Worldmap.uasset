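; BP_Worldmap is a world map actor that shows the player's position and heading with a marker component, PlaneRotator.
; Each Tick it remaps the player pawn's world X and Y from the MapSizeX and MapSizeY extents onto the map's local range, clamped at the edges, to place the marker.
; The marker's yaw copies the pawn's world yaw, with pitch and roll held flat.
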(event `self.ReceiveTick`
  (params (DeltaSeconds :type "Float (single-precision)"))
  (bind (_returnvalue_x _returnvalue_y) (`KismetMathLibrary.BreakVector` (`SceneComponent.K2_GetComponentLocation` (`Actor.RootComponent` (`GameplayStatics.GetPlayerPawn` 0)))))
  (bind (_returnvalue_roll _returnvalue_pitch _returnvalue_yaw) (`KismetMathLibrary.BreakRotator` (`SceneComponent.K2_GetComponentRotation` (`Actor.RootComponent` (`GameplayStatics.GetPlayerPawn` 0)))))
  (`SceneComponent.K2_SetRelativeLocation` (`self.PlaneRotator`) (`KismetMathLibrary.MakeVector` (`KismetMathLibrary.MapRangeClamped` _returnvalue_x (- 0.0 (`self.MapSize_X`)) (`self.MapSize_X`) -50.0 50.0) (`KismetMathLibrary.MapRangeClamped` _returnvalue_y (- 0.0 (`self.MapSize_Y`)) (`self.MapSize_Y`) -50.0 50.0) 1.0) false false)
  (`SceneComponent.K2_SetRelativeRotation` (`self.PlaneRotator`) (`KismetMathLibrary.MakeRotator` 0.0 0.0 _returnvalue_yaw) false false))

(fn `UserConstructionScript`)